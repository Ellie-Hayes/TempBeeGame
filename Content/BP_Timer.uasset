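; BP_Timer is a game timer actor that counts elapsed seconds and shows them through a WBP_TimerWidget it creates on BeginPlay.
; It binds to BP_TopDownGameMode's game started and finished events, and starts counting immediately if BP_HexGrid has AutoSpawnHive set.
; StartTimer re-arms itself every second, incrementing CurrentTime and broadcasting OnTimeChanged.
; StopTimer pauses the stored timer handle.
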(event `self.ReceiveBeginPlay`
  (bind _asbp_top_down_game_mode (cast `/Game/TopDown/Blueprints/BP_TopDownGameMode` (`GameplayStatics.GetGameMode`)))
  (bind _output_get (set `self.GamemodeRef` _asbp_top_down_game_mode))
  (add `/Game/TopDown/Blueprints/BP_TopDownGameMode.OnGameStarted` _output_get (`|CreateDelegate` :!event `Start Timer`))
  (add `/Game/TopDown/Blueprints/BP_TopDownGameMode.OnGameFinished` (`self.GamemodeRef`) (`|CreateDelegate` :!event `StopTimer`))
  (set `self.CurrentTime` 0.0)
  (bind _returnvalue (`|CreateWidget` "/Game/UI/WBP_TimerWidget.WBP_TimerWidget_C"))
  (`/Game/UI/WBP_TimerWidget.Initialise` _returnvalue self)
  (`UserWidget.AddToViewport` _returnvalue 0)
  (bind _returnvalue_2 (`GameplayStatics.GetActorOfClass` "/Game/Hexagon/BP_HexGrid.BP_HexGrid_C"))
  (if (`/Game/Hexagon/BP_HexGrid.AutoSpawnHive?` _returnvalue_2)
    (`self.Start Timer`))
  (`self.OnTimeChanged` 0.0))

(event `Start Timer`
  (bind _returnvalue (`KismetSystemLibrary.K2_SetTimerDelegate` (delegate `Start Timer`) 1.0))
  (set `self.TimerHandleRef` _returnvalue)
  (bind _result (`/Engine/EditorBlueprintResources/StandardMacros.IncrementFloat` (`self.CurrentTime`))
    (:`  `
      (`self.OnTimeChanged` _result))))

(event `StopTimer`
  (`KismetSystemLibrary.K2_PauseTimerHandle` (`self.TimerHandleRef`)))

(fn `UserConstructionScript`)