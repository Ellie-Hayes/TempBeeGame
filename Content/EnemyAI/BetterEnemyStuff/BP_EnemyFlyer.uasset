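; Flying enemy AI pawn that moves to the nearest target and damages it repeatedly on a delay.
; WallBreakerTargeting draws targets from a class priority list; otherwise a repeating sphere trace collects Tower-tagged actors and moves use randomized XY offsets.
; Break events restart nearest-target selection when a move fails or the attack loop's validity check fails.
; Older hive and target-following logic remains, disconnected.
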(event `self.ReceiveBeginPlay`
  (bind (_returnvalue_x _returnvalue_y) (`KismetMathLibrary.BreakVector` (`self.K2_GetActorLocation` (`self.Actor To Attack`))))
  (bind (_returnvalue_x_2 _returnvalue_y_2 _returnvalue_z) (`KismetMathLibrary.BreakVector` (`self.K2_GetActorLocation` self)))
  (bind (_returnvalue_x_3 _returnvalue_y_3) (`KismetMathLibrary.BreakVector` (`self.K2_GetActorLocation` (`self.Actor To Attack`))))
  (if (`self.WallBreakerTargeting?`)
    (for _array_element (`self.ActorTypePriority`)
      (bind _output_get (set `self.Actor Class` _array_element))
      (bind _outactors (`GameplayStatics.GetAllActorsOfClass` _output_get))
      (set `self.Target Actors` _outactors)
      (for _array_element_2 (`self.Target Actors`) :!label _label
        (if (`self.First Loop`)
          (bind _returnvalue (`KismetMathLibrary.Vector_Distance` (`self.K2_GetActorLocation`) (`SceneComponent.K2_GetComponentLocation` (`Actor.RootComponent` _array_element_2))))
          (set `self.Distance` _returnvalue)
          (set `self.First Loop` false)
          (set `self.Actor To Attack` _array_element_2)
          (elif (< _returnvalue (`self.Distance`))
            (set `self.Distance` _returnvalue)
            (set `self.Actor To Attack` _array_element_2))))
      (`|AIMoveTo` self (`KismetMathLibrary.MakeVector` (+ _returnvalue_x 0.0) (+ _returnvalue_y 0.0)) null 125.0
        (:`OnSuccess`
          (`GameplayStatics.ApplyDamage` (`self.Actor To Attack`) 5.0 :!label _label_2)
          (`KismetSystemLibrary.Delay` (`self.AttackDelay`))
          (if (`KismetSystemLibrary.IsValid` _array_element_2)
            (goto _label_2)
            (else
              (`self.Break`))))
        (:`OnFail`
          (`self.Break`))))
    (else
      (`self.Update Targets`)
      (`KismetSystemLibrary.K2_SetTimerDelegate` (delegate `Update Targets`) 5.0 true)
      (for _array_element_3 (`self.Target Actors`) :!label _label_3
        (if (`self.First Loop`)
          (bind _returnvalue_2 (`KismetMathLibrary.Vector_Distance` (`self.K2_GetActorLocation`) (`SceneComponent.K2_GetComponentLocation` (`Actor.RootComponent` _array_element_3))))
          (set `self.Distance` _returnvalue_2)
          (set `self.First Loop` false)
          (set `self.Actor To Attack` _array_element_3)
          (elif (< _returnvalue_2 (`self.Distance`))
            (set `self.Distance` _returnvalue_2)
            (set `self.Actor To Attack` _array_element_3))))
      (`|AIMoveTo` self (`KismetMathLibrary.MakeVector` (+ _returnvalue_x_3 (`KismetMathLibrary.RandomFloatInRange` -35.0 35.0)) (+ _returnvalue_y_3 (`KismetMathLibrary.RandomFloatInRange` -35.0 35.0)) _returnvalue_z) null 150.0
        (:`OnSuccess`
          (`GameplayStatics.ApplyDamage` (`self.Actor To Attack`) 5.0 :!label _label_4)
          (if (`KismetSystemLibrary.IsValid` _array_element_3)
            (`KismetSystemLibrary.Delay` (`self.AttackDelay`))
            (goto _label_4)
            (else
              (`self.Break 2`))))
        (:`OnFail`
          (`self.Break 2`))))))

(event `Break`
  (set `self.First Loop` true)
  (bind _outactors (`GameplayStatics.GetAllActorsOfClass` (`self.Actor Class`)))
  (set `self.Target Actors` _outactors)
  (goto _label))

(event `Update Targets`
  (bind _target_actors (`self.Target Actors`))
  (bind _returnvalue (`self.K2_GetActorLocation` self))
  (bind _outhits (`KismetSystemLibrary.SphereTraceMultiForObjects` _returnvalue _returnvalue 5000.0 (`self.Object Types`)))
  (for _array_element _outhits
    (for _array_element_2 _target_actors
      (bind _returnvalue_2 (and (!= _array_element_2 (`.HitActor` (`GameplayStatics.BreakHitResult` _array_element))) (`self.ActorHasTag` (`.HitActor` (`GameplayStatics.BreakHitResult` _array_element)) "Tower")))
      (if (not _returnvalue_2)
        (break)))
    (if _returnvalue_2
      (`KismetArrayLibrary.Array_Add` _target_actors (`.HitActor` (`GameplayStatics.BreakHitResult` _array_element))))))

(event `Break 2`
  (set `self.First Loop` true)
  (goto _label_3))

(event `Set Enemy Target`
  (params (`Target Actor` :type "Actor Object Reference") (`Hive Location` :type "Vector Structure"))
  ;[1 1 1] Old Code
)

(fn `UserConstructionScript`)