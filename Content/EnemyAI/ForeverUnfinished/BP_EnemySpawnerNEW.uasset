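; Enemy spawner actor that emits timed waves of ant or flying enemies from its own position, with flying enemies placed at a set height.
; SpawnEnemyWave loops through a Delay of wave time divided by the remaining count, so gaps lengthen as the wave progresses.
; Debug keys T and Y trigger ant and flying test waves.
; BeginPlay tags the spawner as Enemy and Snemy when the player character's SpawnerSnemy flag is set.
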(event Custom|SpawnEnemyWave
  (params (Enemy%20Type%20to%20Spawn :type E_EnemyTypes%20Enum :default "NewEnumerator0") (Wave%20Time :type Float%20%28double-precision%29) (Enemies%20To%20Spawn :type Integer))
  (bind _returnvalue (/ Wave%20Time Enemies%20To%20Spawn))
  (bind _self self)
  (bind _returnvalue_2 (Transformation|GetActorTransform _self))
  (Variables|Default|SetEnemies%20to%20Spawn Enemies%20To%20Spawn)
  (if (== Enemy%20Type%20to%20Spawn 0)
    (Game|SpawnActorfromClass (Variables|Default|GetAnt%20Enemy%20Class%20Ref) (Math|Transform|MakeTransform (.location (Transformation|GetActorTransform _self)) (.rotation _returnvalue_2) "1.000000,1.000000,1.000000") "Undefined" "MultiplyWithRoot" 0 0 :!label _label)
    (bind _result (Math|Integer|DecrementInt (Variables|Default|GetEnemies%20to%20Spawn))
      (:%20%20
        (bind _output_get (Variables|Default|SetEnemies%20to%20Spawn _result))
        (if (not (<= _output_get 0))
          (Utilities|FlowControl|Delay _returnvalue)
          (goto _label))))
    (elif (== Enemy%20Type%20to%20Spawn 1)
      (Game|SpawnActorfromClass (Variables|Default|GetFlying%20Enemy%20Class%20Ref) (Math|Transform|MakeTransform (Math|Vector|MakeVector (.x (.location _returnvalue_2)) (.y (.location _returnvalue_2)) (Variables|Default|GetFlying%20Enemy%20Spawn%20Z)) (.rotation _returnvalue_2) "1.000000,1.000000,1.000000") "AdjustIfPossibleButAlwaysSpawn" "MultiplyWithRoot" 0 0 :!label _label_2)
      (bind _result_2 (Math|Integer|DecrementInt (Variables|Default|GetEnemies%20to%20Spawn))
        (:%20%20
          (bind _output_get_2 (Variables|Default|SetEnemies%20to%20Spawn _result_2))
          (if (not (<= _output_get_2 0))
            (Utilities|FlowControl|Delay _returnvalue)
            (goto _label_2)))))))

(event EventBeginPlay
  (bind _asbp_top_down_character (Utilities|Casting|CastToBP_TopDownCharacter (Game|Player|GetPlayerPawn 0)))
  (Variables|Default|SetBoolean_0 (Variables|/Game/TopDown/Blueprints/BP_TopDownCharacter.BP_TopDownCharacter_C|GetSpawnerSnemy _asbp_top_down_character))
  (if (Variables|Default|GetBoolean_0)
    (Variables|Default|SetTags (Utilities|Array|MakeArray (Utilities|Name|MakeLiteralName "Enemy") (Utilities|Name|MakeLiteralName "Snemy")))))

(event Input|KeyboardEvents|DebugKeyT
  (params (Key :type Key%20Structure :default "None") (ActionValue :type Input%20Action%20Value%20Structure))
  (:Pressed
    (CallFunction|SpawnEnemyWave "NewEnumerator0" 6e+01 30)))

(event Input|KeyboardEvents|DebugKeyY
  (params (Key :type Key%20Structure :default "None") (ActionValue :type Input%20Action%20Value%20Structure))
  (:Pressed
    (CallFunction|SpawnEnemyWave "NewEnumerator1" 6e+01 30)))

(fn ConstructionScript)