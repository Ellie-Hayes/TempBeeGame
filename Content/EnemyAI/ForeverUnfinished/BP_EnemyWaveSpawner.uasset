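; Enemy wave spawner actor that spawns a set number of enemies at its own transform, spread over a given wave duration.
; EnemyWave loops through a Delay, adding each spawn to EnemyArray and re-sending EnemyTarget to every enemy in it.
; HiveLocation can be set by event or debug key 8, but enemies always receive a zero hive location.
; Debug key 9 starts a test wave; no other trigger exists here.
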(event Custom|EnemyWave
  (params (Wave%20Time :type Float%20%28double-precision%29) (Enemy%20Count :type Integer))
  (bind _enemy_array (Variables|Default|GetEnemy%20Array))
  (Variables|Default|SetEnemies%20Left%20To%20Spawn Enemy%20Count)
  (bind _returnvalue (Game|SpawnActorfromClass (Variables|Default|GetEnemy%20Class%20Ref) (Transformation|GetActorTransform) "Undefined" "MultiplyWithRoot" 0 0 :!label _label))
  (Utilities|Array|Add _enemy_array _returnvalue)
  (for _array_element _enemy_array
    (Default|SetEnemyTarget _array_element (Variables|Default|GetEnemy%20Target) "0, 0, 0"))
  (bind _result (Math|Integer|DecrementInt (Variables|Default|GetEnemies%20Left%20To%20Spawn))
    (:%20%20
      (bind _output_get (Variables|Default|SetEnemies%20Left%20To%20Spawn _result))
      (if (not (== _output_get 0))
        (Utilities|FlowControl|Delay (/ Wave%20Time Enemy%20Count))
        (goto _label)))))

(event Custom|Set%20Hive%20Location
  (params (Hive%20Location :type Vector))
  (Variables|Default|SetHive%20Location Hive%20Location))

(event EventBeginPlay)

(event Collision|EventActorBeginOverlap
  (params (OtherActor :type Actor%20Object%20Reference)))

(event EventTick
  (params (DeltaSeconds :type Float%20%28single-precision%29)))

(event Input|KeyboardEvents|DebugKey9
  (params (Key :type Key%20Structure) (ActionValue :type Input%20Action%20Value%20Structure))
  (:Pressed
    (CallFunction|EnemyWave 6e+01 30)))

(event Input|KeyboardEvents|DebugKey8
  (params (Key :type Key%20Structure) (ActionValue :type Input%20Action%20Value%20Structure))
  (:Pressed
    (Variables|Default|SetHive%20Location "500.000000,200.000000,480.000000")))

(fn ConstructionScript)