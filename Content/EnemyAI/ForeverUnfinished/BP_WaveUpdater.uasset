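; BP_WaveUpdater is an enemy wave director that binds to the top-down game mode's game-started event and spends an intensity budget on ants, flies and beetles.
; ContinueSpawning recursively makes random picks through CostCheck until the budget runs short, then sends tallies to BP_EnemySpawnerNEW actors.
; NextRound refills a raised budget after a delay, while a timer widens the enemy pool.
; Tallies never reset, and beetles spawn using the ant enum value.
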(event `self.ReceiveBeginPlay`
  (bind _asbp_top_down_game_mode (cast `/Game/TopDown/Blueprints/BP_TopDownGameMode` (`GameplayStatics.GetGameMode`)))
  (add `/Game/TopDown/Blueprints/BP_TopDownGameMode.OnGameStarted` _asbp_top_down_game_mode (`|CreateDelegate` :!event `Initialise`)))

(event `ContinueSpawning`
  (bind _returnvalue (`KismetMathLibrary.RandomInteger` (`self.CurrentEnemyTypes`)))
  (if (== _returnvalue 0) :!label _label
    (bind _canafford_ (`self.CostCheck` (`self.AntCost`)))
    (`/Engine/EditorBlueprintResources/StandardMacros.IncrementInt` (`self.AntsToSpawn`)
      (:`  `
        (if _canafford_
          (`self.ContinueSpawning` :!label _label_2)
          (else
            (`self.Spawn Enemies` :!label _label_3)
            (set `self.CurrentRoundIntensity` (+ (`self.CurrentRoundIntensity`) 5))
            (`self.NextRound`)))))
    (elif (== _returnvalue 1)
      (bind _canafford__2 (`self.CostCheck` (`self.FlyCost`)))
      (`/Engine/EditorBlueprintResources/StandardMacros.IncrementInt` (`self.FlysToSpawn`)
        (:`  `
          (if _canafford__2
            (goto _label_2)
            (else
              (goto _label_3)))))
      (elif (== _returnvalue 2)
        (bind _canafford__3 (`self.CostCheck` (`self.BeetleCost`)))
        (`/Engine/EditorBlueprintResources/StandardMacros.IncrementInt` (`self.BeetlesToSpawn`)
          (:`  `
            (if _canafford__3
              (goto _label_2)
              (else
                (goto _label_3)))))))))

(event `NextRound`
  (set `self.RoundIntensity` (`self.CurrentRoundIntensity`))
  (`KismetSystemLibrary.Delay` 30.0)
  (goto _label))

(event `Initialise`
  (`KismetSystemLibrary.K2_SetTimerDelegate` (delegate `IncreaseEnemyTypes`) 40.0)
  (bind _outactors (`GameplayStatics.GetAllActorsOfClass` "/Game/EnemyAI/ForeverUnfinished/BP_EnemySpawnerNEW.BP_EnemySpawnerNEW_C"))
  (goto _label))

(event `Spawn Enemies`
  (for _array_element (stale `Initialise` _outactors)
    (`/Game/EnemyAI/ForeverUnfinished/BP_EnemySpawnerNEW.SpawnEnemyWave` _array_element "NewEnumerator0" 9.0 (`self.AntsToSpawn`))
    (`/Game/EnemyAI/ForeverUnfinished/BP_EnemySpawnerNEW.SpawnEnemyWave` _array_element "NewEnumerator1" 9.0 (`self.FlysToSpawn`))
    (`/Game/EnemyAI/ForeverUnfinished/BP_EnemySpawnerNEW.SpawnEnemyWave` _array_element "NewEnumerator0" 9.0 (`self.BeetlesToSpawn`))))

(event `IncreaseEnemyTypes`
  (bind _currentenemytypes (`self.CurrentEnemyTypes`))
  (`/Engine/EditorBlueprintResources/StandardMacros.IncrementInt` _currentenemytypes
    (:`  `
      (`KismetSystemLibrary.Delay` 40.0)
      (`/Engine/EditorBlueprintResources/StandardMacros.IncrementInt` _currentenemytypes))))

(fn `CostCheck`
  (params (Cost :type Integer))
  (returns (`CanAfford?` :type Boolean))
  (bind _roundintensity (`self.RoundIntensity`))
  (bind _returnvalue (>= _roundintensity Cost))
  (if _returnvalue
    (set `self.RoundIntensity` (- _roundintensity Cost)))
  (return _returnvalue))

(fn `UserConstructionScript`)