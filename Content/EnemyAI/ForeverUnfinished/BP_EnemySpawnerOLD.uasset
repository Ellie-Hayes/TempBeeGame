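; Legacy enemy spawner actor that fills a group of enemies at a spawn point and points them at a shared target.
; On BeginPlay it spawns the configured class about once a second, storing each enemy in an array until the maximum count is reached.
; A looping Delay then re-sends the target to every stored enemy each second, with a zeroed hive location.
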(event `self.ReceiveBeginPlay`
  (bind _enemy_array (`self.Enemy Array`))
  (bind (_returnvalue_location _returnvalue_rotation) (`KismetMathLibrary.BreakTransform` (`SceneComponent.K2_GetComponentToWorld` (`self.SpawnPoint`))))
  (bind _returnvalue (`|SpawnActorFromClass` (`self.EnemyClassToSpawn`) (`KismetMathLibrary.MakeTransform` _returnvalue_location _returnvalue_rotation) "Undefined" "MultiplyWithRoot" null null :!label _label))
  (`KismetArrayLibrary.Array_Add` _enemy_array _returnvalue)
  (bind _result (`/Engine/EditorBlueprintResources/StandardMacros.IncrementInt` (`self.EnemyCount`))
    (:`  `
      (`KismetSystemLibrary.Delay` 1.0)
      (if (>= _result (`self.EnemyMaxCount`))
        (for _array_element _enemy_array :!label _label_2
          (`/Game/EnemyAI/ForeverUnfinished/BP_EnemyAIBase.Set Enemy Target` _array_element (`self.Enemy Target Obj`) (0.0 0.0 0.0))
          (`KismetSystemLibrary.Delay` 1.0 :!label _label_3)
          (goto _label_2))
        (goto _label_3)
        (else
          (goto _label))))))

(fn `UserConstructionScript`)