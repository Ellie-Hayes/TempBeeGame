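; Enemy spawner that runs escalating waves of ants, flies and beetles, hooking into the game mode's game-start event.
; NewWaveData takes override counts or spends a round-scaled budget, currently only on ants because the beetle and fly purchase branches are disconnected.
; After a wave delay, it spawns at random navmesh points around itself in timed steps, then immediately starts the next wave.
; The outer-ring hex tile location helper is unused.
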(event `self.ReceiveBeginPlay`
  (bind _asbp_top_down_game_mode (cast `/Game/TopDown/Blueprints/BP_TopDownGameMode` (`GameplayStatics.GetGameMode`)))
  (add `/Game/TopDown/Blueprints/BP_TopDownGameMode.OnGameStarted` _asbp_top_down_game_mode (`|CreateDelegate` :!event `Init`))
  (bind _returnvalue (`GameplayStatics.GetActorOfClass` "/Game/Hexagon/BP_HexGrid.BP_HexGrid_C"))
  (set `self.GridRef` _returnvalue))

(event `Init`
  (bind _returnvalue (`GameplayStatics.GetActorOfClass` "/Script/NavigationSystem.RecastNavMesh"))
  (set `self.Nav Data` _returnvalue)
  (`self.New Wave`))

(event `ContinueSpawning`
  (bind _antstospawn (`self.AntsToSpawn`))
  (bind _flystospawn (`self.FlysToSpawn`))
  (bind _beetlestospawn (`self.BeetlesToSpawn`))
  (`KismetSystemLibrary.Delay` 0.2)
  (if (> _antstospawn 0) :!label _label
    (`self.Spawn Ant`)
    (`/Engine/EditorBlueprintResources/StandardMacros.DecrementInt` _antstospawn
      (:`  `
        _)))
  (if (> _flystospawn 0)
    (`self.Spawn Fly`)
    (`/Engine/EditorBlueprintResources/StandardMacros.DecrementInt` _flystospawn
      (:`  `
        _)))
  (if (> _beetlestospawn 0)
    (`self.Spawn Beetle`)
    (`/Engine/EditorBlueprintResources/StandardMacros.DecrementInt` _beetlestospawn
      (:`  `
        _)))
  (if (or (> (`self.AntsToSpawn`) 0) (> (`self.FlysToSpawn`) 0) (> (`self.BeetlesToSpawn`) 0))
    (`self.ContinueSpawning`)
    (else
      (`self.New Wave`))))

(event `New Wave`
  (`self.New Wave Data` (struct))
  (`KismetSystemLibrary.Delay` (`self.Wave Delay`))
  (goto _label))

(event `Spawn Ant`
  (bind _randomlocation (`NavigationSystemV1.K2_GetRandomReachablePointInRadius` (`self.K2_GetActorLocation`) (`self.RandomSpawnRadius`) (`self.Nav Data`) null))
  (`|SpawnActorFromClass` (`self.Ant Actor Ref`) (`KismetMathLibrary.MakeTransform` (`KismetMathLibrary.MakeVector` (.x _randomlocation) (.y _randomlocation) (+ (.z _randomlocation) 50.0))) "AlwaysSpawn" "MultiplyWithRoot" null null))

(event `Spawn Fly`
  (bind _randomlocation (`NavigationSystemV1.K2_GetRandomReachablePointInRadius` (`self.K2_GetActorLocation`) 200.0 (`self.Nav Data`) null))
  (`|SpawnActorFromClass` (`self.Fly Actor Ref`) (`KismetMathLibrary.MakeTransform` (`KismetMathLibrary.MakeVector` (.x _randomlocation) (.y _randomlocation) 5000.0)) "Undefined" "MultiplyWithRoot" null null))

(event `Spawn Beetle`
  (`|SpawnActorFromClass` (`self.Beetle Actor Ref`) (`KismetMathLibrary.MakeTransform` (`NavigationSystemV1.K2_GetRandomReachablePointInRadius` (`self.K2_GetActorLocation`) 200.0 (`self.Nav Data`) null)) "Undefined" "MultiplyWithRoot" null null))

(fn `GetSpawnLocation`
  (returns (RandomLoc :type "Vector Structure"))
  (locals (RandomStream :type "RandomStream Structure"))
  (bind _outerringtiles (`/Game/Hexagon/BP_HexGrid.OuterRingTiles` (`self.GridRef`)))
  (bind _returnvalue (`KismetMathLibrary.RandomIntegerInRangeFromStream` (`local.RandomStream`) 0 (- (`KismetArrayLibrary.Array_Length` _outerringtiles) 1)))
  (`KismetMathLibrary.SeedRandomStream` (`local.RandomStream`))
  (`KismetSystemLibrary.PrintString` (`KismetStringLibrary.Conv_IntToString` _returnvalue))
  (return (`KismetMathLibrary.MakeVector` (.x (`self.K2_GetActorLocation` (`|GetArrayItem` _outerringtiles _returnvalue))) (.y (`self.K2_GetActorLocation` (`|GetArrayItem` _outerringtiles _returnvalue))) (+ (.z (`self.K2_GetActorLocation` (`|GetArrayItem` _outerringtiles _returnvalue))) 100.0))))

(fn `New Wave Data`
  (params (WaveOverride :type "/Game/EnemyAI/S_EnemyCount Structure"))
  (set `self.AntsToSpawn` 0)
  (set `self.FlysToSpawn` 0)
  (set `self.BeetlesToSpawn` 0)
  (`/Engine/EditorBlueprintResources/StandardMacros.IncrementInt` (`self.Round`)
    (:`  `
      (if (> (`self.Round`) 2)
        (set `self.Enemy2Unlocked?` true))
      (if (> (`self.Round`) 4)
        (set `self.Enemy3Unlocked?` true))
      (if (or (> WaveOverride_AntCount_2_758D5D3F4CA9DD10A98539B2E69C95D9 0) (> WaveOverride_FlyCount_5_313A8C3F4ED1F912DEB885A03B609371 0) (> WaveOverride_BeetleCount_6_C051673F430ED584033EDDB9DCD8DA07 0))
        (set `self.AntsToSpawn` WaveOverride_AntCount_2_758D5D3F4CA9DD10A98539B2E69C95D9)
        (set `self.FlysToSpawn` WaveOverride_FlyCount_5_313A8C3F4ED1F912DEB885A03B609371)
        (set `self.BeetlesToSpawn` WaveOverride_BeetleCount_6_C051673F430ED584033EDDB9DCD8DA07)
        (else
          (set `self.MaxWaveCost` (* (`self.Round`) (`self.WaveSizeMultiplier`)))
          (if (>= (`self.MaxWaveCost`) (`self.Ant Cost`)) :!label _label
            (set `self.MaxWaveCost` (- (`self.MaxWaveCost`) (`self.Ant Cost`)))
            (`/Engine/EditorBlueprintResources/StandardMacros.IncrementInt` (`self.AntsToSpawn`)
              (:`  `
                (goto _label)))
            (else
              _))))
      (return))))

(fn `UserConstructionScript`)