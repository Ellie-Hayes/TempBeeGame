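; Enemy spawner that spawns five data-driven waves at its own transform, repeating the fifth indefinitely, with B as a debug trigger.
; BeginPlay binds to the game mode's OnGameStarted; Init starts the wave chain.
; SpawnWave hands each enemy entry to the first free of five delayed-loop spawners, the fifth taking overflow.
; Waves are spaced by the largest per-enemy interval plus a grace period; spawner 3 loops only when it raises that maximum.
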(event Custom|Init
  (CallFunction|WaveTimer))

(event Custom|Spawn%20Wave
  (params (Wave%20Data :type S%20Wave%20Data%20Structure))
  (for _array_element (.enemydata Wave%20Data)
    (if (Variables|Default|GetFreeSpawner1?)
      (Variables|Default|SetEnemyType1 (.enemytype _array_element))
      (CallFunction|SpawnEnemies1)
      (elif (Variables|Default|GetFreeSpawner2?)
        (Variables|Default|SetEnemyType2 (.enemytype _array_element))
        (CallFunction|SpawnEnemies2)
        (elif (Variables|Default|GetFreeSpawner3?)
          (Variables|Default|SetEnemyType3 (.enemytype _array_element))
          (CallFunction|SpawnEnemies3)
          (elif (Variables|Default|GetFreeSpawner4?)
            (Variables|Default|SetEnemyType4 (.enemytype _array_element))
            (CallFunction|SpawnEnemies4)
            (else
              (Variables|Default|SetEnemyType5 (.enemytype _array_element))
              (CallFunction|SpawnEnemies5))))))))

(event Custom|Spawn%20Enemies%201
  (bind _returnvalue (Transformation|GetActorTransform))
  (Variables|Default|SetFreeSpawner1? false)
  (bind _output_get (Variables|Default|SetDelay1 (/ (.enemyspawntime (stale Custom|Spawn%20Wave _array_element)) (.enemycount (stale Custom|Spawn%20Wave _array_element)))))
  (if (> _output_get (Variables|Default|GetCurrent%20Longest%20to%20Spawn))
    (Variables|Default|SetCurrent%20Longest%20to%20Spawn _output_get))
  (Utilities|ForLoopwithDelay 1 (.enemycount (stale Custom|Spawn%20Wave _array_element)) _output_get
    (:Loop%20Body
      (Game|SpawnActorfromClass (Variables|Default|GetEnemyType1) (Math|Transform|MakeTransform (.location _returnvalue) (.rotation _returnvalue) "1.000000,1.000000,1.000000") "Undefined" "MultiplyWithRoot" 0 0))
    (:Completed
      (Variables|Default|SetFreeSpawner1? true))))

(event Custom|Spawn%20Enemies%202
  (bind _returnvalue (Transformation|GetActorTransform))
  (Variables|Default|SetFreeSpawner2? false)
  (bind _output_get (Variables|Default|SetDelay2 (/ (.enemyspawntime (stale Custom|Spawn%20Wave _array_element)) (.enemycount (stale Custom|Spawn%20Wave _array_element)))))
  (if (> _output_get (Variables|Default|GetCurrent%20Longest%20to%20Spawn))
    (Variables|Default|SetCurrent%20Longest%20to%20Spawn _output_get))
  (Utilities|ForLoopwithDelay 1 (.enemycount (stale Custom|Spawn%20Wave _array_element)) _output_get
    (:Loop%20Body
      (Game|SpawnActorfromClass (Variables|Default|GetEnemyType2) (Math|Transform|MakeTransform (.location _returnvalue) (.rotation _returnvalue) "1.000000,1.000000,1.000000") "Undefined" "MultiplyWithRoot" 0 0))
    (:Completed
      (Variables|Default|SetFreeSpawner2? true))))

(event Custom|Spawn%20Enemies%203
  (bind _returnvalue (Transformation|GetActorTransform))
  (Variables|Default|SetFreeSpawner3? false)
  (bind _output_get (Variables|Default|SetDelay3 (/ (.enemyspawntime (stale Custom|Spawn%20Wave _array_element)) (.enemycount (stale Custom|Spawn%20Wave _array_element)))))
  (if (> _output_get (Variables|Default|GetCurrent%20Longest%20to%20Spawn))
    (Variables|Default|SetCurrent%20Longest%20to%20Spawn _output_get)
    (Utilities|ForLoopwithDelay 1 (.enemycount (stale Custom|Spawn%20Wave _array_element)) _output_get
      (:Loop%20Body
        (Game|SpawnActorfromClass (Variables|Default|GetEnemyType3) (Math|Transform|MakeTransform (.location _returnvalue) (.rotation _returnvalue) "1.000000,1.000000,1.000000") "Undefined" "MultiplyWithRoot" 0 0))
      (:Completed
        (Variables|Default|SetFreeSpawner3? true)))))

(event Custom|Spawn%20Enemies%204
  (bind _returnvalue (Transformation|GetActorTransform))
  (Variables|Default|SetFreeSpawner4? false)
  (bind _output_get (Variables|Default|SetDelay4 (/ (.enemyspawntime (stale Custom|Spawn%20Wave _array_element)) (.enemycount (stale Custom|Spawn%20Wave _array_element)))))
  (if (> _output_get (Variables|Default|GetCurrent%20Longest%20to%20Spawn))
    (Variables|Default|SetCurrent%20Longest%20to%20Spawn _output_get))
  (Utilities|ForLoopwithDelay 1 (.enemycount (stale Custom|Spawn%20Wave _array_element)) _output_get
    (:Loop%20Body
      (Game|SpawnActorfromClass (Variables|Default|GetEnemyType4) (Math|Transform|MakeTransform (.location _returnvalue) (.rotation _returnvalue) "1.000000,1.000000,1.000000") "Undefined" "MultiplyWithRoot" 0 0))
    (:Completed
      (Variables|Default|SetFreeSpawner4? true))))

(event Custom|Spawn%20Enemies%205
  (bind _returnvalue (Transformation|GetActorTransform))
  (bind _output_get (Variables|Default|SetDelay5 (/ (.enemyspawntime (stale Custom|Spawn%20Wave _array_element)) (.enemycount (stale Custom|Spawn%20Wave _array_element)))))
  (if (> _output_get (Variables|Default|GetCurrent%20Longest%20to%20Spawn))
    (Variables|Default|SetCurrent%20Longest%20to%20Spawn _output_get))
  (Utilities|ForLoopwithDelay 1 (.enemycount (stale Custom|Spawn%20Wave _array_element)) _output_get
    (:Loop%20Body
      (Game|SpawnActorfromClass (Variables|Default|GetEnemyType5) (Math|Transform|MakeTransform (.location _returnvalue) (.rotation _returnvalue) "1.000000,1.000000,1.000000") "Undefined" "MultiplyWithRoot" 0 0))))

(event Custom|Wave%20Timer
  (bind _current_longest_to_spawn (Variables|Default|GetCurrent%20Longest%20to%20Spawn))
  (bind _wavegraceperiod (Variables|Default|GetWaveGracePeriod))
  (bind _returnvalue (+ _current_longest_to_spawn _wavegraceperiod))
  (CallFunction|SpawnWave (Variables|Default|GetWave%201%20Data))
  (Utilities|FlowControl|Delay _returnvalue)
  (CallFunction|SpawnWave (Variables|Default|GetWave%202%20Data))
  (Utilities|FlowControl|Delay _returnvalue)
  (CallFunction|SpawnWave (Variables|Default|GetWave%203%20Data))
  (Utilities|FlowControl|Delay _returnvalue)
  (CallFunction|SpawnWave (Variables|Default|GetWave%204%20Data))
  (Utilities|FlowControl|Delay _returnvalue :!label _label)
  (CallFunction|SpawnWave (Variables|Default|GetWave%205%20Data))
  (goto _label))

(event EventBeginPlay
  (bind _asbp_top_down_game_mode (Utilities|Casting|CastToBP_TopDownGameMode (Game|GetGameMode)))
  (EventDispatchers|BindEventtoOnGameStarted _asbp_top_down_game_mode (EventDispatchers|CreateEvent :!event Custom|Init)))

(event Input|KeyboardEvents|DebugKeyB
  (params (Key :type Key%20Structure :default "None") (ActionValue :type Input%20Action%20Value%20Structure))
  (bind _current_longest_to_spawn (Variables|Default|GetCurrent%20Longest%20to%20Spawn))
  (bind _wavegraceperiod (Variables|Default|GetWaveGracePeriod))
  (bind _returnvalue (+ _current_longest_to_spawn _wavegraceperiod))
  (:Pressed
    (CallFunction|SpawnWave (Variables|Default|GetWave%201%20Data))
    (Utilities|FlowControl|Delay _returnvalue)
    (CallFunction|SpawnWave (Variables|Default|GetWave%202%20Data))
    (Utilities|FlowControl|Delay _returnvalue)
    (CallFunction|SpawnWave (Variables|Default|GetWave%203%20Data))
    (Utilities|FlowControl|Delay _returnvalue)
    (CallFunction|SpawnWave (Variables|Default|GetWave%204%20Data))
    (Utilities|FlowControl|Delay _returnvalue :!label _label)
    (CallFunction|SpawnWave (Variables|Default|GetWave%205%20Data))
    (goto _label)))

(fn ConstructionScript)