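; Wave director that buys enemy spawns from a round intensity budget and sends them through every BP_EnemySpawnerNEW.
; It binds to the game mode's game-started event, and ContinueSpawning recursively picks random ant, fly or beetle costs until one is unaffordable.
; NextRound then refills a budget raised each round and resumes after a delay.
; A timer widens the random type range twice, though the beetle branch spawns the ant branch's enum value.
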(event `self.ReceiveBeginPlay`
  (bind _asbp_top_down_game_mode (cast `/Game/TopDown/Blueprints/BP_TopDownGameMode` (`GameplayStatics.GetGameMode`)))
  (add `/Game/TopDown/Blueprints/BP_TopDownGameMode.OnGameStarted` _asbp_top_down_game_mode (`|CreateDelegate` :!event `Initialise`)))

(event `ContinueSpawning`
  (bind _returnvalue (`KismetMathLibrary.RandomInteger` (`self.CurrentEnemyTypes`)))
  (if (== _returnvalue 0) :!label _label
    (bind _canafford_ (`self.CostCheck` (`self.AntCost`)))
    (if _canafford_
      (for _array_element (stale `Initialise` _outactors)
        (`/Game/EnemyAI/BP_EnemySpawnerNEW.SpawnEnemyWave` _array_element "NewEnumerator0" 2.5 1))
      (`self.ContinueSpawning` :!label _label_2)
      (else
        (set `self.CurrentRoundIntensity` (+ (`self.CurrentRoundIntensity`) 10) :!label _label_3)
        (`self.NextRound`)))
    (elif (== _returnvalue 1)
      (bind _canafford__2 (`self.CostCheck` (`self.FlyCost`)))
      (if _canafford__2
        (for _array_element_2 (stale `Initialise` _outactors)
          (`/Game/EnemyAI/BP_EnemySpawnerNEW.SpawnEnemyWave` _array_element_2 "NewEnumerator1" 2.5 1))
        (goto _label_2)
        (else
          (goto _label_3)))
      (elif (== _returnvalue 2)
        (bind _canafford__3 (`self.CostCheck` (`self.BeetleCost`)))
        (if _canafford__3
          (for _array_element_3 (stale `Initialise` _outactors)
            (`/Game/EnemyAI/BP_EnemySpawnerNEW.SpawnEnemyWave` _array_element_3 "NewEnumerator0" 2.5 1))
          (goto _label_2)
          (else
            (goto _label_3)))))))

(event `NextRound`
  (set `self.RoundIntensity` (`self.CurrentRoundIntensity`))
  (`KismetSystemLibrary.Delay` 10.0)
  (goto _label))

(event `Initialise`
  (`KismetSystemLibrary.K2_SetTimerDelegate` (delegate `IncreaseEnemyTypes`) 40.0)
  (bind _outactors (`GameplayStatics.GetAllActorsOfClass` "/Game/EnemyAI/BP_EnemySpawnerNEW.BP_EnemySpawnerNEW_C"))
  (goto _label))

(event `IncreaseEnemyTypes`
  (bind _currentenemytypes (`self.CurrentEnemyTypes`))
  ;[1 1 1] Every 30 seconds, increment the amount of enemies we are spawning by 1 (actually 6)
  (`/Engine/EditorBlueprintResources/StandardMacros.IncrementInt` _currentenemytypes
    (:`  `
      (`KismetSystemLibrary.Delay` 40.0)
      (`/Engine/EditorBlueprintResources/StandardMacros.IncrementInt` _currentenemytypes))))

(fn `CostCheck`
  (params (Cost :type Integer))
  (returns (`CanAfford?` :type Boolean))
  (bind _roundintensity (`self.RoundIntensity`))
  (bind _returnvalue (>= _roundintensity Cost))
  (if _returnvalue
    (bind _output_get (set `self.RoundIntensity` (- _roundintensity Cost)))
    (`KismetSystemLibrary.PrintString` (`KismetStringLibrary.Conv_IntToString` _output_get)))
  (return _returnvalue))

(fn `UserConstructionScript`)