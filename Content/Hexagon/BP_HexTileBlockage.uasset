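; BP_HexTileBlockage is a blockage tile for the hexagon grid, with a Niagara component that serves as its fog.
; SetInitialSpawnValues stores the grid generator reference, tile coordinates and ring data, then takes its activated state from that ring.
; The fog shows only on non-activated tiles with ShowFog enabled.
; IsSelectedNeighbour is left empty, so the tile does nothing on that event.
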(event `self.IsSelectedNeighbour`)

(fn `SetInitialSpawnValues`
  (params (TileData :type "/Game/Hexagon/S_TileData Structure") (`Grid Generator Ref` :type "/Game/Hexagon/BP_HexGrid Object Reference"))
  (bind (_tilecoordinates _ringdata) (break `/Game/Hexagon/S_TileData` TileData))
  (set `self.Grid Generator Ref` `Grid Generator Ref`)
  (set `self.TileCoordinates` _tilecoordinates)
  (bind _output_get (set `self.Ring Data` _ringdata))
  (set `self.Activated` (`.TilesAreActivated?_17_5F031C0142DA9C60351E38989C1D1E3E` (break `/Game/Hexagon/S_RingData` _output_get)))
  (`SceneComponent.SetVisibility` (`self.Niagara`) (not (`self.Activated`)) false)
  (if (not (`self.ShowFog`))
    (`SceneComponent.SetVisibility` (`self.Niagara`) false false)))

(fn `UserConstructionScript`
  (`parent.UserConstructionScript`))