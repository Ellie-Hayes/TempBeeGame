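; Generates the hexagonal tile map at BeginPlay and tracks placed towers and their connection to the hive.
; Builds row-based coordinates in ratio-sized rings, whose probabilities pick gaps, blockages, multipliers or base tiles, spaced by mesh bounds.
; Places enemy spawners at four cardinal edge tiles and can auto-spawn the hive, starting the game.
; When a tower is eaten, a capped breadth-first search from the hive updates each tower's connected flag.
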(event `self.ReceiveBeginPlay`
  (bind _asbp_top_down_game_mode (cast `/Game/TopDown/Blueprints/BP_TopDownGameMode` (`GameplayStatics.GetGameMode`)))
  (set `self.GamemodeRef` _asbp_top_down_game_mode)
  (`self.GenerateNewGrid`))

(event `PlacedTile`
  (params (TileConstructed :type "/Game/Towers/BP_BasePlaceable Object Reference"))
  (if (== (`GameplayStatics.GetObjectClass` TileConstructed) "/Game/Towers/FlowerFields/BP_FlowerField.BP_FlowerField_C")
    (`/Engine/EditorBlueprintResources/StandardMacros.IncrementInt` (`self.FlowerFieldCount`))
    (else
      (`KismetArrayLibrary.Array_Add` (`self.ActiveTowers`) TileConstructed)
      (`self.OnTIlePlaced` TileConstructed))))

(event `TowerEaten`
  (params (DestroyedTower :type "/Game/Towers/BP_BasePlaceable Object Reference"))
  (`KismetArrayLibrary.Array_RemoveItem` (`self.ActiveTowers`) DestroyedTower)
  (`self.OnTowerEaten` DestroyedTower)
  (bind _connectedtiles (`self.FindConnectedTileToBaseHive`))
  (bind _output_get (set `self.VisitedTowers` _connectedtiles))
  (`self.SetConnectedTiles` _output_get))

(fn `AdjustRadius`
  (bind _combinedratio (`self.GetCombinedRatios`))
  (bind _returnvalue (mod (`self.Radius`) _combinedratio))
  (if (not (== _returnvalue 0))
    (set `self.Radius` (+ (- _combinedratio _returnvalue) (`self.Radius`)))))

(fn `CheckShouldGenerateSpecialTile`
  (params (TileData :type "/Game/Hexagon/S_TileData Structure"))
  (returns (TileClassToSpawn :type "/Game/Hexagon/BP_BaseHexTile Class Reference") (ShouldSpawn :type Boolean))
  (locals (TempTileClassToSpawn :type "/Game/Hexagon/BP_BaseHexTile Class Reference"))
  (bind (_tilecoordinates _ringdata) (break `/Game/Hexagon/S_TileData` TileData))
  (bind _multipliertiles (`self.MultiplierTiles`))
  (bind (_name _index _blockagetileprobability _multipliertileprobability _chompedtileprobability) (break `/Game/Hexagon/S_RingData` _ringdata))
  (for _array_element (`self.Enemy Spawner Coords`)
    (if (== _array_element _tilecoordinates)
      (return "/Game/Hexagon/BP_BaseHexTile.BP_BaseHexTile_C" true)))
  (if (<= (`KismetMathLibrary.RandomFloatInRange` 0.0 100.0) _chompedtileprobability)
    (return null false)
    (elif (<= (`KismetMathLibrary.RandomFloatInRange` 0.0 100.0) _blockagetileprobability)
      (return "/Game/Hexagon/BP_HexTileBlockage.BP_HexTileBlockage_C" true)
      (elif (<= (`KismetMathLibrary.RandomFloatInRange` 0.0 100.0) _multipliertileprobability)
        (return (`|GetArrayItem` _multipliertiles (`KismetMathLibrary.RandomIntegerInRange` 0 (- (`KismetArrayLibrary.Array_Length` _multipliertiles) 1))) true)
        (else
          (return "/Game/Hexagon/BP_BaseHexTile.BP_BaseHexTile_C" true))))))

(fn `CheckTileRing`
  (params (SingleRingUnit :type "Float (double-precision)") (CurrentRowLength :type Integer) (RowID :type Integer) (CurrentTileIndex :type Integer))
  (returns (RingData :type "/Game/Hexagon/S_RingData Structure"))
  (locals (CurrentTileRingOffset :type "Float (double-precision)" :default 0.0))
  (bind (_arrayindex _arrayelement) (`/Engine/EditorBlueprintResources/StandardMacros.ReverseForEachLoop` (`self.RingDatas`))
    (:`LoopBody`
      (bind _returnvalue (* (`local.SingleRingUnit`) (`.Ratio_13_7799C16E45327B6E6883859FF136F837` (break `/Game/Hexagon/S_RingData` _arrayelement))))
      (bind _returnvalue_2 (+ _returnvalue (`local.CurrentTileRingOffset`)))
      (if (or (> (`local.RowID`) (- (`self.Radius`) _returnvalue_2)) (< (`local.CurrentTileIndex`) _returnvalue_2) (> (`local.CurrentTileIndex`) (- (`local.CurrentRowLength`) _returnvalue_2)) (< (`local.RowID`) (+ (* (`self.Radius`) -1) _returnvalue_2)))
        (return _arrayelement)
        (else
          (set `local.CurrentTileRingOffset` (+ (`local.CurrentTileRingOffset`) _returnvalue)))))))

(fn `CheckTileRingCentral`
  (params (SingleRingUnit :type "Float (double-precision)") (CurrentTileIndex :type Integer))
  (returns (RingData :type "/Game/Hexagon/S_RingData Structure"))
  (locals (CurrentTileRingOffset :type "Float (double-precision)" :default 0.0))
  (for _array_element (`self.RingDatas`)
    (bind _returnvalue (* (`local.SingleRingUnit`) (`.Ratio_13_7799C16E45327B6E6883859FF136F837` (break `/Game/Hexagon/S_RingData` _array_element))))
    (bind _returnvalue_2 (+ _returnvalue (`local.CurrentTileRingOffset`)))
    (if (and (<= (`local.CurrentTileIndex`) _returnvalue_2) (>= (`local.CurrentTileIndex`) (- 0 _returnvalue_2)))
      (return _array_element)
      (else
        (set `local.CurrentTileRingOffset` (+ _returnvalue (`local.CurrentTileRingOffset`)))))))

(fn `CreateEnemySpawnerCoords`
  (returns (EnemySpawnerCoords :type "Array of Vector Structure"))
  (locals (Coords :type "Array of Vector Structure"))
  (bind _coords (`local.Coords`))
  (`KismetArrayLibrary.Array_Add` _coords (`KismetMathLibrary.MakeVector` 0.0 0.0 (`KismetMathLibrary.Conv_IntToDouble` (`self.Radius`))))
  (`KismetArrayLibrary.Array_Add` _coords (`KismetMathLibrary.MakeVector` 0.0 0.0 (`KismetMathLibrary.Conv_IntToDouble` (* (`self.Radius`) -1))))
  (`KismetArrayLibrary.Array_Add` _coords (`KismetMathLibrary.MakeVector` (`KismetMathLibrary.Conv_IntToDouble` (* (`self.Radius`) -1))))
  (`KismetArrayLibrary.Array_Add` _coords (`KismetMathLibrary.MakeVector` (`KismetMathLibrary.Conv_IntToDouble` (`self.Radius`))))
  (return (`local.Coords`)))

(fn `FindConnectedTileToBaseHive`
  (returns (ConnectedTiles :type "Array of /Game/Hexagon/BP_BaseHexTile Object Reference"))
  (locals (ToVisit :type "Array of /Game/Hexagon/BP_BaseHexTile Object Reference") (Visited :type "Array of /Game/Hexagon/BP_BaseHexTile Object Reference") (Current :type "/Game/Hexagon/BP_BaseHexTile Object Reference") (CappedInt :type Integer))
  (bind _current (`local.Current`))
  (`KismetArrayLibrary.Array_Add` (`local.ToVisit`) (`/Game/TopDown/Blueprints/BP_TopDownGameMode.HiveLocation` (`self.GamemodeRef`)))
  (while (and (`KismetArrayLibrary.Array_IsNotEmpty` (`local.ToVisit`)) (< (`local.CappedInt`) 300))
    (`/Engine/EditorBlueprintResources/StandardMacros.IncrementInt` (`local.CappedInt`)
      (:`  `
        (bind _output_get (set `local.Current` (`|GetArrayItem` (`local.ToVisit`))))
        (`KismetArrayLibrary.Array_RemoveItem` (`local.ToVisit`) _output_get)
        (if (not (`KismetArrayLibrary.Array_Contains` (`local.Visited`) (`local.Current`)))
          (`KismetArrayLibrary.Array_Add` (`local.Visited`) (`local.Current`))
          (if (`KismetArrayLibrary.Array_IsEmpty` (`/Game/Hexagon/BP_BaseHexTile.Tile Neighbours` (`local.Current`)))
            (`KismetSystemLibrary.PrintString` "No tile neighbours calculating")
            (`/Game/Hexagon/BP_BaseHexTile.SetTileNeighbours` _current))
          (for _array_element (`/Game/Hexagon/BP_BaseHexTile.Tile Neighbours` _current)
            (if (and (`KismetSystemLibrary.IsValid` (`/Game/Hexagon/BP_BaseHexTile.PlacedTile` _array_element)) (not (`KismetArrayLibrary.Array_Contains` (`local.Visited`) _array_element)))
              (`KismetArrayLibrary.Array_Add` (`local.ToVisit`) _array_element)))))))
  (return (`local.Visited`)))

(fn `GenerateCentralRow`
  (locals (TempCoords :type "Vector Structure") (SingleRingUnit :type "Float (double-precision)"))
  ;[1 1 1] Center row has to be calculated seperately because the other rows are based on whether they are above or below 0
  (set `local.SingleRingUnit` (/ (`self.Radius`) (`self.GetCombinedRatios`)))
  (for _index (range (`self.Radius`))
    (bind _returnvalue (+ _index 1))
    (set `local.TempCoords` (`KismetMathLibrary.MakeVector` 0.0 0.0 (`KismetMathLibrary.Conv_IntToDouble` _returnvalue)))
    (bind _ringdata (`self.CheckTileRingCentral` (`local.SingleRingUnit`) _returnvalue))
    (`KismetArrayLibrary.Array_Add` (`self.TileDatas`) (make `/Game/Hexagon/S_TileData` (`local.TempCoords`) _ringdata))
    (bind _returnvalue_2 (- (* _index -1) 1))
    (set `local.TempCoords` (`KismetMathLibrary.MakeVector` 0.0 0.0 (`KismetMathLibrary.Conv_IntToDouble` _returnvalue_2)))
    (bind _ringdata_2 (`self.CheckTileRingCentral` (`local.SingleRingUnit`) _returnvalue_2))
    (`KismetArrayLibrary.Array_Add` (`self.TileDatas`) (make `/Game/Hexagon/S_TileData` (`local.TempCoords`) _ringdata_2))))

(fn `GenerateNewGrid`
  (bind _returnvalue (`StaticMesh.GetBoundingBox` (`self.StaticMesh`)))
  (`self.AdjustRadius`)
  ;[1 1 1] Calculates automatic offset using bounding boxes of given mesh
  (bind _result (`/Engine/EditorBlueprintResources/StandardMacros.NegateFloat` (.x (break `Box` _returnvalue)))
    (:`  `
      (set `self.CalcOffset` (+ _result (.x (`.Max` (break `Box` _returnvalue)))))
      ;[1 1 1] Adds center tile
      (`KismetArrayLibrary.Array_Add` (`self.TileDatas`) (make `/Game/Hexagon/S_TileData` (0.0 0.0 0.0) (`|GetArrayItem` (`self.RingDatas`))))
      (`self.GenerateCentralRow`)
      (`self.GenerateRemainingRows`)
      (bind _enemyspawnercoords (`self.CreateEnemySpawnerCoords`))
      (set `self.Enemy Spawner Coords` _enemyspawnercoords)
      (`self.PlaceTiles`)
      (`self.SpawnCardinalDirectionsEnemySpawners`)
      (if (`self.AutoSpawnHive?`)
        (for _array_element (`self.SpawnedTiles`)
          (if (and (`KismetMathLibrary.EqualExactly_VectorVector` (`/Game/Hexagon/BP_BaseHexTile.TileCoordinates` _array_element) (`self.HiveSpawnLocation`)) (not (`/Game/TopDown/Blueprints/BP_TopDownGameMode.GameStarted` (`self.GamemodeRef`))))
            (bind _newtile (`self.OverrideSpawnTileType` "/Game/Hexagon/BP_BaseHexTile.BP_BaseHexTile_C" _array_element))
            (`/Game/Hexagon/BP_BaseHexTile.PlaceTile` _newtile "/Game/Towers/BP_BaseResourceGenerator.BP_BaseResourceGenerator_C")
            (`/Game/TopDown/Blueprints/BP_TopDownGameMode.StartGame` (`self.GamemodeRef`) _newtile)))))))

(fn `GenerateRemainingRows`
  (locals (RowsRemaining :type Integer) (HorizontalDisplacement :type "Float (double-precision)") (VerticalDisplacement :type "Float (double-precision)") (CurrentRowLength :type Integer) (RowID :type Integer) (TempCoords :type "Vector Structure" :default (0.0 0.0 0.0)) (CurrentTileDataOffset :type Integer) (SingleTileRingUnit :type "Float (double-precision)") (CurrentTileIndex :type Integer))
  (set `local.SingleTileRingUnit` (/ (`self.Radius`) (`self.GetCombinedRatios`)))
  (set `local.RowsRemaining` (- (* (`self.Radius`) 2) 1))
  (set `local.CurrentRowLength` (* (`self.Radius`) 2))
  ;[1 1 1] Runs the loop for each row remaining
  (for _index (range (+ (`local.RowsRemaining`) 1))
    (bind _output_get (set `local.RowID` _index))
    ;[1 1 1] If past half the rows (on the lower half of the ring), reset variables
    (if (== _output_get (`self.Radius`))
      (set `local.HorizontalDisplacement` 0.0)
      (set `local.VerticalDisplacement` 0.0)
      (set `local.CurrentRowLength` (* (`self.Radius`) 2)))
    (set `local.HorizontalDisplacement` (+ (`local.HorizontalDisplacement`) 0.5))
    ;[1 1 1] If above the center row, make Y coordinate positive, else make it negative
    (`/Engine/EditorBlueprintResources/StandardMacros.DecrementInt` (`local.CurrentRowLength`)
      (:`  `
        (if (< (`local.RowID`) (`self.Radius`))
          (set `local.VerticalDisplacement` (+ (`local.VerticalDisplacement`) 1.0))
          (else
            (set `local.VerticalDisplacement` (+ (`local.VerticalDisplacement`) -1.0))))
        ;[1 1 1] Construct final coordinates
        (for _index_2 (range (+ (`local.CurrentRowLength`) 1))
          (set `local.CurrentTileIndex` _index_2)
          (set `local.TempCoords` (`KismetMathLibrary.MakeVector` (`local.VerticalDisplacement`) 0.0 (- (`self.Radius`) _index_2 (`local.HorizontalDisplacement`))))
          (bind _ringdata (`self.CheckTileRing` (`local.SingleTileRingUnit`) (`local.CurrentRowLength`) (`KismetMathLibrary.FTrunc` (`local.VerticalDisplacement`)) (`local.CurrentTileIndex`)))
          (`KismetArrayLibrary.Array_Add` (`self.TileDatas`) (make `/Game/Hexagon/S_TileData` (`local.TempCoords`) _ringdata)))))))

(fn `GenerateRingSpecific`
  (params (RingIndex :type Integer) (MaxAmount :type Integer))
  (returns (FoundTiles :type "Array of /Game/Hexagon/BP_BaseHexTile Object Reference") (AllRingTiles :type "Array of /Game/Hexagon/BP_BaseHexTile Object Reference"))
  (locals (RingTIles :type "Array of /Game/Hexagon/BP_BaseHexTile Object Reference") (TilesToPlaceOn :type "Array of /Game/Hexagon/BP_BaseHexTile Object Reference") (CurrentAmount :type Integer) (CurrentTileToCheck :type "/Game/Hexagon/BP_BaseHexTile Object Reference") (RandNumber :type Integer))
  (for _array_element (`self.SpawnedTiles`)
    (if (and (== (`.Index_27_7F7EF94543C7283639EFCBA35A5ADF17` (break `/Game/Hexagon/S_RingData` (`/Game/Hexagon/BP_BaseHexTile.Ring Data` _array_element))) (`local.RingIndex`)) (!= (`GameplayStatics.GetObjectClass` _array_element) "/Game/Hexagon/BP_HexTileBlockage.BP_HexTileBlockage_C"))
      (`KismetArrayLibrary.Array_Add` (`local.RingTIles`) _array_element)))
  (for _ (range (+ (`local.MaxAmount`) 1))
    (bind _output_get (set `local.RandNumber` (`KismetMathLibrary.RandomIntegerInRange` 0 (- (`KismetArrayLibrary.Array_Length` (`local.RingTIles`)) 1))))
    (set `local.CurrentTileToCheck` (`|GetArrayItem` (`local.RingTIles`) _output_get))
    (`KismetArrayLibrary.Array_Add` (`local.TilesToPlaceOn`) (`local.CurrentTileToCheck`))
    (`KismetArrayLibrary.Array_RemoveItem` (`local.RingTIles`) (`local.CurrentTileToCheck`))
    (bind _result (`/Engine/EditorBlueprintResources/StandardMacros.IncrementInt` (`local.CurrentAmount`))
      (:`  `
        (if (>= _result (`local.MaxAmount`))
          (return (`local.TilesToPlaceOn`) (`local.RingTIles`)))))))

(fn `GetCombinedRatios`
  (returns (CombinedRatio :type Integer))
  (locals (TempCombinedRatio :type Integer))
  (for _array_element (`self.RingDatas`)
    (set `local.TempCombinedRatio` (+ (`.Ratio_13_7799C16E45327B6E6883859FF136F837` (break `/Game/Hexagon/S_RingData` _array_element)) (`local.TempCombinedRatio`))))
  (return (`local.TempCombinedRatio`)))

(fn `GetTileNeighboursByTile`
  (params (Tile :type "/Game/Hexagon/BP_BaseHexTile Object Reference"))
  (returns (TileNeighbours :type "Array of /Game/Hexagon/BP_BaseHexTile Object Reference"))
  (locals (TempTileNeighbours :type "Array of /Game/Hexagon/BP_BaseHexTile Object Reference") (TempCoords :type "Vector Structure" :default (0.0 0.0 0.0)) (NeighbourCoordsToUse :type "Array of Vector2D Structure"))
  (bind _output_get (set `local.TempCoords` (`/Game/Hexagon/BP_BaseHexTile.TileCoordinates` Tile)))
  (if (== (mod (.x _output_get) 2.0) 0.0)
    (set `local.NeighbourCoordsToUse` (`self.NeighbourCoordListEven`))
    (else
      (set `local.NeighbourCoordsToUse` (`self.NeighbourCoordListOdd`))))
  (for _array_element (`self.SpawnedTiles`)
    (for _array_element_2 (`local.NeighbourCoordsToUse`)
      (bind (_x _y) (`KismetMathLibrary.BreakVector2D` _array_element_2))
      (if (== (`/Game/Hexagon/BP_BaseHexTile.TileCoordinates` _array_element) (`KismetMathLibrary.MakeVector` (+ _x (.x (`local.TempCoords`))) 0.0 (+ _y (.z (`local.TempCoords`)))) :`ErrorTolerance` 0.1)
        (`KismetArrayLibrary.Array_Add` (`local.TempTileNeighbours`) _array_element))))
  (return (`local.TempTileNeighbours`)))

(fn `OverrideSpawnTileType`
  (params (NewType :type "/Game/Hexagon/BP_BaseHexTile Class Reference") (TileToOverride :type "/Game/Hexagon/BP_BaseHexTile Object Reference"))
  (returns (NewTile :type "/Game/Hexagon/BP_BaseHexTile Object Reference"))
  (bind _spawnedtiles (`self.SpawnedTiles`))
  (bind _returnvalue (`|SpawnActorFromClass` NewType (`self.GetTransform` TileToOverride) "AlwaysSpawn" "MultiplyWithRoot" null null))
  (`KismetArrayLibrary.Array_Add` _spawnedtiles _returnvalue)
  (`KismetArrayLibrary.Array_RemoveItem` _spawnedtiles (`local.TileToOverride`))
  (`/Game/Hexagon/BP_BaseHexTile.SetInitialSpawnValues` _returnvalue (make `/Game/Hexagon/S_TileData` (`/Game/Hexagon/BP_BaseHexTile.TileCoordinates` TileToOverride) (`/Game/Hexagon/BP_BaseHexTile.Ring Data` TileToOverride)) self)
  (return _returnvalue))

(fn `PlaceTiles`
  (bind _scale (`self.Scale`))
  (bind _returnvalue (* (`self.CalcOffset`) (`self.Scale`)))
  ;[1 1 1] Just a lot of math to take into account scale, offset etc to calculate the location to place the tile
  (for _array_element (`self.TileDatas`)
    (bind (_tileclasstospawn _shouldspawn) (`self.CheckShouldGenerateSpecialTile` _array_element))
    (if _shouldspawn
      (bind _x (.x (`.TileCoordinates_2_8D4B45914E30AE369213128CE0649578` (break `/Game/Hexagon/S_TileData` _array_element))))
      (bind _returnvalue_2 (`|SpawnActorFromClass` _tileclasstospawn (`KismetMathLibrary.MakeTransform` (`KismetMathLibrary.MakeVector` (* (* (* _x _returnvalue) (`self.OffsetMultiplier`)) 0.86) (* (* (.z (`.TileCoordinates_2_8D4B45914E30AE369213128CE0649578` (break `/Game/Hexagon/S_TileData` _array_element))) _returnvalue) (`self.OffsetMultiplier`))) (struct :`Yaw` 30.0) (`KismetMathLibrary.MakeVector` _scale _scale _scale)) "AlwaysSpawn" "MultiplyWithRoot" null null))
      ;[1 1 1] More math to adjust location if its on an even row because thats just how hexagons work apparently
      (`/Game/Hexagon/BP_BaseHexTile.SetInitialSpawnValues` _returnvalue_2 _array_element self)
      (`KismetArrayLibrary.Array_Add` (`self.SpawnedTiles`) _returnvalue_2)
      (if (== (mod _x 2.0) 0.0)
        (`self.K2_SetActorLocation` _returnvalue_2 (`KismetMathLibrary.MakeVector` (.x (`self.K2_GetActorLocation` _returnvalue_2)) (+ (.y (`self.K2_GetActorLocation` _returnvalue_2)) (/ (* (`self.CalcOffset`) (`self.Scale`)) 2.0)) (.z (`self.K2_GetActorLocation` _returnvalue_2))) false false)))))

(fn `RandomlySpawnEnemySpawners`
  (if (> (`self.MaxEnemySpawners`) 0)
    (bind (_foundtiles _allringtiles) (`self.GenerateRingSpecific` 3 (`self.MaxEnemySpawners`)))
    (set `self.OuterRingTiles` _allringtiles)
    (for _array_element _foundtiles
      (`/Engine/EditorBlueprintResources/StandardMacros.IsValid` _array_element
        (:`Is Valid`
          (bind _newtile (`self.OverrideSpawnTileType` "/Game/Hexagon/BP_BaseHexTile.BP_BaseHexTile_C" _array_element))
          (`/Game/Hexagon/BP_BaseHexTile.PlaceEnemySpawner` _newtile))))))

(fn `SetConnectedTiles`
  (params (ConnectedTiles :type "Array of /Game/Hexagon/BP_BaseHexTile Object Reference"))
  (locals (CurrentTower :type "/Game/Towers/BP_BasePlaceable Object Reference"))
  (for _array_element (`self.ActiveTowers`)
    (set `local.CurrentTower` _array_element)
    (if (`KismetArrayLibrary.Array_Contains` (`local.ConnectedTiles`) (`/Game/Towers/BP_BasePlaceable.Owning Tile` _array_element))
      (set `/Game/Towers/BP_BasePlaceable.ConnectedToHive` true (`local.CurrentTower`))
      (else
        (set `/Game/Towers/BP_BasePlaceable.ConnectedToHive` false (`local.CurrentTower`))))))

(fn `SpawnCardinalDirectionsEnemySpawners`
  (for _array_element (`self.SpawnedTiles`)
    (for _array_element_2 (`self.Enemy Spawner Coords`)
      (if (`KismetMathLibrary.EqualExactly_VectorVector` (`/Game/Hexagon/BP_BaseHexTile.TileCoordinates` _array_element) _array_element_2)
        (`/Game/Hexagon/BP_BaseHexTile.PlaceEnemySpawner` _array_element)))))

(fn `UserConstructionScript`)