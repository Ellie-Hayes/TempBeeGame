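; BP_FlowerTower is a tower that generates nectar for the player through the top-down game mode.
; BeginPlay caches the game mode and starts a looping timer for nectar generation.
; AddNectar pays out only while connected to a hive, using the truncated value of the tower's second attribute.
; Windmill buff events toggle a flag that adds a bonus to each payout.
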(event `self.ReceiveBeginPlay`
  (`parent.ReceiveBeginPlay`)
  (bind _asbp_top_down_game_mode (cast `/Game/TopDown/Blueprints/BP_TopDownGameMode` (`GameplayStatics.GetGameMode`)))
  (set `self.GamemodeRef` _asbp_top_down_game_mode)
  (`KismetSystemLibrary.K2_SetTimerDelegate` (`|CreateDelegate` :!event `AddNectar`) (`self.TimeBetweenNectarGenerate`) true))

(event `AddNectar`
  (bind _gamemoderef (`self.GamemodeRef`))
  (bind _returnvalue (`KismetMathLibrary.FTrunc` (`.CurrentAmount_20_1C1F45344E87F293D251F4BC53114A3C` (break `/Game/F_TowerAttributes` (`|GetArrayItem` (`self.Attributes`) 1)))))
  (if (`self.ConnectedToHive`)
    (if (`self.Windmill Buff`)
      (`/Game/TopDown/Blueprints/BP_TopDownGameMode.ChangeNectarAmount` _gamemoderef (+ _returnvalue (`self.Windmill Buff Addition`)) true)
      (else
        (`/Game/TopDown/Blueprints/BP_TopDownGameMode.ChangeNectarAmount` _gamemoderef _returnvalue true)))))

(event `Windmill Buff Apply`
  (set `self.Windmill Buff` true))

(event `Windmill Buff Remove`
  (set `self.Windmill Buff` false))

(fn `UserConstructionScript`
  (`parent.UserConstructionScript`))