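; Tower manager that keeps a registry of placed towers by type: pollen bombers, single turrets, honey traps, jelly boosters and the base hive.
; It binds to the hex grid's tile-placed and tower-eaten events on BeginPlay.
; Placed tiles are sorted by a class-cast switch, then wrapped into a combined array of tower-type structs and broadcast.
; Removal searches that combined array, while hive removal only casts the game mode, with no further action.
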(event `self.ReceiveBeginPlay`
  (bind _returnvalue (`GameplayStatics.GetActorOfClass` "/Game/Hexagon/BP_HexGrid.BP_HexGrid_C"))
  (add `/Game/Hexagon/BP_HexGrid.OnTIlePlaced` _returnvalue (`|CreateDelegate` :!event `CheckTilePlaced`))
  (add `/Game/Hexagon/BP_HexGrid.OnTowerEaten` _returnvalue (`|CreateDelegate` :!event `RemoveTiles`)))

(fn `CheckContains`
  (params (ArrayToCheck :type "Array of /Game/Towers/BP_BasePlaceable Object Reference") (Item :type "/Game/Towers/BP_BasePlaceable Object Reference"))
  (returns (`Contained?` :type Boolean))
  (if (`KismetArrayLibrary.Array_Contains` ArrayToCheck Item)
    (`KismetArrayLibrary.Array_RemoveItem` (`local.ArrayToCheck`) (`local.Item`))
    (return true)
    (else
      (return false))))

(fn `CheckTilePlaced`
  (params (TilePlaced :type "/Game/Towers/BP_BasePlaceable Object Reference"))
  (locals (PlacedTile :type "/Game/Towers/BP_BasePlaceable Object Reference"))
  (bind _output_get (set `local.PlacedTile` TilePlaced))
  (`self.SwitchOnClass` _output_get
    (:`PollenBomber`
      (`KismetArrayLibrary.Array_Add` (`self.PollenBombers`) (`local.PlacedTile`)))
    (:`SingleTurret`
      (`KismetArrayLibrary.Array_Add` (`self.SingleTurret`) (`local.PlacedTile`)))
    (:`Hive`
      (set `self.BaseHive` (`local.PlacedTile`)))
    (:`HoneyTrap`
      (`KismetArrayLibrary.Array_Add` (`self.HoneyTraps`) (`local.PlacedTile`)))
    (:`JellyBooster`
      (`KismetArrayLibrary.Array_Add` (`self.JellyBoosters`) (`local.PlacedTile`))))
  (`self.UpdateArrays`)
  (`self.OnArraysUpdated`))

(fn `RemoveTiles`
  (params (TilesRemoves :type "/Game/Towers/BP_BasePlaceable Object Reference"))
  (locals (RemovedTiles :type "/Game/Towers/BP_BasePlaceable Object Reference"))
  (if (== TilesRemoves (`self.BaseHive`))
    (cast `/Game/TopDown/Blueprints/BP_TopDownGameMode` (`GameplayStatics.GetGameMode`))
    (else
      (set `local.RemovedTiles` TilesRemoves)
      (for _array_element (`self.AllTowerArrays`)
        (bind _contained_ (`self.CheckContains` (`.Array_3_3909278B4BAAE9F4DDF5278688441E8C` (break `/Game/Towers/F_TowerTypes` _array_element)) (`local.RemovedTiles`)))
        (if _contained_
          (`self.UpdateArrays`)
          (return))))))

(fn `UpdateArrays`
  (set `self.AllTowerArrays` (`|MakeArray` (make `/Game/Towers/F_TowerTypes` (`self.PollenBombers`)) (make `/Game/Towers/F_TowerTypes` (`self.SingleTurret`)) (make `/Game/Towers/F_TowerTypes` (`self.HoneyTraps`)) (make `/Game/Towers/F_TowerTypes` (`self.JellyBoosters`)) (make `/Game/Towers/F_TowerTypes` (`|MakeArray` (`self.BaseHive`))))))

(fn `UserConstructionScript`)