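; Honey trap tower that slows enemies while they stand inside its Box trigger.
; On overlap, tagged BP_EnemyAITest actors have walk speed multiplied by the third attribute, then restored on exit from one OriginalSpeed variable shared across all enemies.
; UpgradeStat extends the parent and calls UpdateStat, which multiplies the box's current X and Y scale by the first attribute, so repeated upgrades compound.
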(event `Update Stat`
  (bind _box (`self.Box`))
  (bind (_relativescale3d_x _relativescale3d_y _relativescale3d_z) (`KismetMathLibrary.BreakVector` (`SceneComponent.RelativeScale3D` _box)))
  (bind ((`AttributeType_27_401693E34E656CC35BD962A172F4A6D6` _attributetype) (`CurrentAmount_20_1C1F45344E87F293D251F4BC53114A3C` _currentamount)) (break `/Game/F_TowerAttributes` (`|GetArrayItem` (`self.Attributes`))))
  (`SceneComponent.SetRelativeScale3D` _box (`KismetMathLibrary.MakeVector` (* _relativescale3d_x _currentamount) (* _relativescale3d_y _currentamount) _relativescale3d_z)))

(event `self.Box.OnComponentBeginOverlap`
  (params (OverlappedComponent :type "PrimitiveComponent Object Reference") (OtherActor :type "Actor Object Reference") (OtherComp :type "PrimitiveComponent Object Reference") (OtherBodyIndex :type Integer) (bFromSweep :type Boolean) (SweepResult :type "HitResult Structure (by ref)"))
  (if (`self.ActorHasTag` OtherActor "Enemy")
    (bind _asbp_enemy_aitest (cast `/Game/EnemyAI/BP_EnemyAITest` OtherActor))
    (bind _output_get (set `self.As BP Enemy AITest` _asbp_enemy_aitest))
    (set `self.Original Speed` (`MovementComponent.GetMaxSpeed` (`Character.CharacterMovement` _output_get)))
    (set `CharacterMovementComponent.MaxWalkSpeed` (* (`self.Original Speed`) (`.CurrentAmount_20_1C1F45344E87F293D251F4BC53114A3C` (break `/Game/F_TowerAttributes` (`|GetArrayItem` (`self.Attributes`) 2)))) (`Character.CharacterMovement` _output_get))))

(event `self.Box.OnComponentEndOverlap`
  (params (OverlappedComponent :type "PrimitiveComponent Object Reference") (OtherActor :type "Actor Object Reference") (OtherComp :type "PrimitiveComponent Object Reference") (OtherBodyIndex :type Integer))
  (if (`self.ActorHasTag` OtherActor "Enemy")
    (bind _asbp_enemy_aitest (cast `/Game/EnemyAI/BP_EnemyAITest` OtherActor))
    (set `CharacterMovementComponent.MaxWalkSpeed` (`self.Original Speed`) (`Character.CharacterMovement` _asbp_enemy_aitest))))

(fn `UpgradeStat`
  (params (Index :type Integer))
  (`parent.UpgradeStat` Index)
  (`self.Update Stat`))

(fn `UserConstructionScript`)