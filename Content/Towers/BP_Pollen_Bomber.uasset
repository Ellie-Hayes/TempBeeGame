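; Pollen Bomber tower that, while connected to the hive, turns toward enemies seen by PawnSensing and lobs grenades at them, limited by a fire-rate delay.
; MortarPrediction leads the target by velocity and distance, adds random scatter, solves an arced launch velocity and draws debug spheres.
; Upgradeable attributes, scaled by the current multiplier, set sight radius and the value passed to each grenade.
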(event `Update Stat`
  (set `PawnSensingComponent.SightRadius` (* (`.CurrentAmount_20_1C1F45344E87F293D251F4BC53114A3C` (break `/Game/F_TowerAttributes` (`|GetArrayItem` (`self.Attributes`) 1))) (`self.CurrentMultiplier`)) (`self.PawnSensing`)))

(event `self.PawnSensing.OnSeePawn`
  (params (Pawn :type "Pawn Object Reference"))
  (bind (_returnvalue_roll _returnvalue_pitch _returnvalue_yaw) (`KismetMathLibrary.BreakRotator` (`KismetMathLibrary.FindLookAtRotation` (`self.K2_GetActorLocation`) (`self.K2_GetActorLocation` Pawn))))
  (if (`self.ConnectedToHive`)
    (if (`self.ActorHasTag` Pawn "Enemy")
      (`SceneComponent.K2_SetWorldRotation` (`self.Cube1`) (`KismetMathLibrary.MakeRotator` _returnvalue_roll 0.0 _returnvalue_yaw) false false)
      (if (`self.CanShoot?`)
        (bind _velocity (`self.Mortar Prediction` Pawn))
        (set `self.Velocity` _velocity)
        (bind _returnvalue (`|SpawnActorFromClass` "/Game/TD_Prototipings/BP_Granade.BP_Granade_C" (`KismetMathLibrary.MakeTransform` (`SceneComponent.K2_GetComponentLocation` (`self.Arrow`))) "Undefined" "MultiplyWithRoot" self null))
        (`/Game/TD_Prototipings/BP_Granade.Initialise` _returnvalue (* (`.CurrentAmount_20_1C1F45344E87F293D251F4BC53114A3C` (break `/Game/F_TowerAttributes` (`|GetArrayItem` (`self.Attributes`) 2))) (`self.CurrentMultiplier`)))
        (`ProjectileMovementComponent.SetVelocityInLocalSpace` (`/Game/TD_Prototipings/BP_Granade.ProjectileMovement` _returnvalue) (* (`self.Velocity`) 3.0))
        (set `self.CanShoot?` false)
        (if true
          (`KismetSystemLibrary.Delay` (`self.Fire Rate`))
          (set `self.CanShoot?` true))))))

(fn `Add Vector Randomness`
  (params (Vector :type "Vector Structure") (Randomness :type "Float (double-precision)") (`Use X` :type Boolean) (`Use Y` :type Boolean) (`Use Z` :type Boolean))
  (returns (`Randomness Return` :type "Vector Structure"))
  (bind _x (.x Vector))
  (bind _y (.y Vector))
  (bind _z (.z Vector))
  (bind _returnvalue (* Randomness -1.0))
  (return (`KismetMathLibrary.MakeVector` (`KismetMathLibrary.SelectFloat` (+ (`KismetMathLibrary.RandomFloatInRange` _returnvalue Randomness) _x) _x `Use X`) (`KismetMathLibrary.SelectFloat` (+ (`KismetMathLibrary.RandomFloatInRange` _returnvalue Randomness) _y) _y `Use Y`) (`KismetMathLibrary.SelectFloat` (+ (`KismetMathLibrary.RandomFloatInRange` _returnvalue) _z) _z `Use Z`))))

(fn `Mortar Prediction`
  (params (`Target Actor` :type "Actor Object Reference"))
  (returns (Velocity :type "Vector Structure"))
  (locals (`Target Actor Velocity` :type "Vector Structure") (`Target Actor Location` :type "Vector Structure"))
  (bind _returnvalue (+ (`local.Target Actor Location`) (* (`local.Target Actor Velocity`) (/ (`KismetMathLibrary.Vector_Distance` (`local.Target Actor Location`) (`self.K2_GetActorLocation`)) 1200.0))))
  (bind _randomness_return (`self.Add Vector Randomness` _returnvalue (`self.Randomness`) true true true))
  (set `local.Target Actor Velocity` (`self.GetVelocity` `Target Actor`))
  (set `local.Target Actor Location` (`self.K2_GetActorLocation` `Target Actor`))
  (`KismetSystemLibrary.DrawDebugSphere` _returnvalue 100.0 12 (struct :`R` 0.067444 :`G` 1.0 :`A` 1.0) 2.0)
  (`KismetSystemLibrary.DrawDebugSphere` _randomness_return 50.0 12 (struct :`R` 1.0 :`B` 0.087291 :`A` 1.0) 2.0)
  (bind (_outlaunchvelocity _returnvalue_2) (`GameplayStatics.SuggestProjectileVelocity_CustomArc` (`SceneComponent.K2_GetComponentLocation` (`self.Arrow`)) _randomness_return 0.0 0.2))
  (if _returnvalue_2
    (return _outlaunchvelocity)))

(fn `UpgradeStat`
  (params (Index :type Integer))
  (`parent.UpgradeStat` Index)
  (`self.Update Stat`))

(fn `UserConstructionScript`)