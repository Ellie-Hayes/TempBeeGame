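; BP_test is a tower actor that turns toward any pawn it sees and fires BP_Bullet.
; A PawnSensing sighting snaps the whole actor to face the pawn, then spawns the bullet at the Arrow's transform after a short delay.
; The CanShoot flag then gates both turning and firing until a cooldown delay ends.
; BeginPlay, overlap and Tick are unused disabled stubs.
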(event `self.PawnSensing.OnSeePawn`
  (params (Pawn :type "Pawn Object Reference"))
  (if (`self.CanShoot?`)
    (`self.K2_SetActorRotation` (`KismetMathLibrary.FindLookAtRotation` (`self.K2_GetActorLocation`) (`self.K2_GetActorLocation` Pawn)))
    (`KismetSystemLibrary.Delay` 0.2)
    (`|SpawnActorFromClass` "/Game/TD_Prototipings/BP_Bullet.BP_Bullet_C" (`SceneComponent.K2_GetComponentToWorld` (`self.Arrow`)) "Undefined" "MultiplyWithRoot" null null)
    (set `self.CanShoot?` false)
    (`KismetSystemLibrary.Delay` (`self.Duration_0`))
    (set `self.CanShoot?` true)))

(fn `UserConstructionScript`
  (`parent.UserConstructionScript`))