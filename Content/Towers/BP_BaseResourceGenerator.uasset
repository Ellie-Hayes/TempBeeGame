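; BP_BaseResourceGenerator is a tower that generates Nectar over time and ends the game when it dies.
; On BeginPlay it caches BP_TopDownGameMode and starts a looping timer at the configured generation interval.
; AddNectar adds the configured amount through the game mode's ChangeNectarAmount.
; The OnTowerDeath override runs the parent logic, then calls EndGame on the game mode.
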(event `self.ReceiveBeginPlay`
  (bind _asbp_top_down_game_mode (cast `/Game/TopDown/Blueprints/BP_TopDownGameMode` (`GameplayStatics.GetGameMode`)))
  (set `self.GamemodeRef` _asbp_top_down_game_mode)
  (`KismetSystemLibrary.K2_SetTimerDelegate` (`|CreateDelegate` :!event `AddNectar`) (`self.TimeBetweenResourceGenerated`) true))

(event `AddNectar`
  (`/Game/TopDown/Blueprints/BP_TopDownGameMode.ChangeNectarAmount` (`self.GamemodeRef`) (`self.ResourceGenerateAmount`) true))

(fn `OnTowerDeath`
  (`parent.OnTowerDeath`)
  (`/Game/TopDown/Blueprints/BP_TopDownGameMode.EndGame` (`self.GamemodeRef`)))

(fn `UserConstructionScript`)