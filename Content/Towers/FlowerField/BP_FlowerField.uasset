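; BP_FlowerField is a flower field tower that grows over time and produces nectar actors.
; On BeginPlay, two looping timers drive Grow, which doubles each flower mesh's scale per level up to a maximum, and GenerateNectar.
; GenerateNectar spawns BP_Nectar at the Arrow with randomized pitch and yaw, storing it in NectarArray until CurrentNectar equals MaxNectar.
; ResetNectar zeroes that counter, allowing production to resume.
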(event `GenerateNectar`
  (bind _arrow (`self.Arrow`))
  (bind (_returnvalue_roll _returnvalue_pitch _returnvalue_yaw) (`KismetMathLibrary.BreakRotator` (`SceneComponent.K2_GetComponentRotation` _arrow)))
  (if (not (== (`self.CurrentNectar`) (`self.MaxNectar`)))
    ;[1 1 1] SpawnNectarActor
    (set `self.CurrentNectar` (+ (`self.CurrentNectar`) (`self.NectarGenerateAmount`)))
    (bind _offsetrotation (`self.RandomDeviation` _returnvalue_yaw))
    (bind _offsetrotation_2 (`self.RandomDeviation` _returnvalue_pitch))
    (bind _returnvalue (`|SpawnActorFromClass` "/Game/Towers/FlowerField/BP_Nectar.BP_Nectar_C" (`KismetMathLibrary.MakeTransform` (`SceneComponent.K2_GetComponentLocation` _arrow) (`KismetMathLibrary.MakeRotator` _returnvalue_roll _offsetrotation_2 _offsetrotation)) "AlwaysSpawn" "MultiplyWithRoot" null null))
    (`KismetArrayLibrary.Array_Add` (`self.NectarArray`) _returnvalue)))

(event `self.ReceiveBeginPlay`
  (`parent.ReceiveBeginPlay`)
  (`KismetSystemLibrary.K2_SetTimerDelegate` (delegate `Grow`) (`self.GrowTime`) true)
  (`KismetSystemLibrary.K2_SetTimerDelegate` (delegate `GenerateNectar`) (`self.NectarCreateTime`) true)
  (set `self.Flowers` (`|MakeArray` (`self.StaticMesh1`) (`self.StaticMesh2`) (`self.StaticMesh3`) (`self.StaticMesh4`) (`self.StaticMesh5`)))
  (`KismetSystemLibrary.PrintString` "Hello"))

(event `Grow`
  (bind _currentlevel (`self.CurrentLevel`))
  (if (`self.CanLevel`)
    (for _array_element (`self.Flowers`)
      (bind _asstatic_mesh_component (cast `StaticMeshComponent` _array_element))
      (`SceneComponent.SetWorldScale3D` _asstatic_mesh_component (* (`SceneComponent.K2_GetComponentScale` _asstatic_mesh_component) 2)))
    (`/Engine/EditorBlueprintResources/StandardMacros.IncrementInt` _currentlevel
      (:`  `
        (if (== _currentlevel (`self.MaxLevel`))
          (set `self.CanLevel` false))))))

(event `ResetNectar`
  (set `self.CurrentNectar` 0))

(fn `RandomDeviation`
  (params (ArrowRotation :type "Float (double-precision)"))
  (returns (OffsetRotation :type "Float (double-precision)"))
  (return (+ ArrowRotation (`KismetMathLibrary.RandomFloatInRange` 60.0 -60.0))))

(fn `UserConstructionScript`
  (`parent.UserConstructionScript`))