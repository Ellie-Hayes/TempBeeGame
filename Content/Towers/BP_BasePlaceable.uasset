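; Base placeable tower Blueprint that sits on an owning grid tile, takes damage and can be selected by clicking.
; An attribute array supplies max health and upgradeable stats, with upgrades raising cost and firing change events.
; Damage spawns popups and, at zero health, clears the tile, notifies the grid generator and destroys the actor.
; Initialise creates a paused looping heal timer and, if health is enabled, a camera-facing health widget.
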(event `Initialise`
  (params (OwningTile :type "/Game/Hexagon/BP_BaseHexTile Object Reference"))
  (set `self.Owning Tile` OwningTile)
  (set `self.CurrentHealth` (`.CurrentAmount_20_1C1F45344E87F293D251F4BC53114A3C` (break `/Game/F_TowerAttributes` (`self.GetHealthAtrribute` (`self.Attributes`)))))
  (bind _returnvalue (`KismetSystemLibrary.K2_SetTimerDelegate` (delegate `Heal`) 1.0 true))
  (bind _output_get (set `self.Healing Timer` _returnvalue))
  (`KismetSystemLibrary.K2_PauseTimerHandle` _output_get)
  (if (`self.HasHealth`)
    (bind _returnvalue_2 (`GameplayStatics.GetActorOfClass` "/Game/TopDown/Blueprints/BP_TopDownCharacter.BP_TopDownCharacter_C"))
    (bind _output_get_2 (set `self.CharacterRef` _returnvalue_2))
    (add `/Game/TopDown/Blueprints/BP_TopDownCharacter.OnCameraRotated` _output_get_2 (`|CreateDelegate` :!event `RotateHealthWidget`))
    (`self.RotateHealthWidget` (`SceneComponent.K2_GetComponentRotation` (`/Game/TopDown/Blueprints/BP_TopDownCharacter.SpringArm` (`self.CharacterRef`))))
    (bind _aswbp_tower_health (cast `/Game/UI/WBP_TowerHealth` (`WidgetComponent.GetWidget` (`self.WidgetHealth`))))
    (`/Game/UI/WBP_TowerHealth.Initialise` _aswbp_tower_health self)
    (else
      (`SceneComponent.SetVisibility` (`self.WidgetHealth`) false false))))

(event `Heal`
  (if true
    (set `self.CurrentHealth` (`KismetMathLibrary.FClamp` (+ (`self.CurrentHealth`) (`self.HealAmount`)) 0.0 (`.CurrentAmount_20_1C1F45344E87F293D251F4BC53114A3C` (break `/Game/F_TowerAttributes` (`self.GetHealthAtrribute` (`self.Attributes`))))))))

(event `self.ReceiveAnyDamage`
  (params (Damage :type "Float (single-precision)") (DamageType :type "DamageType Object Reference") (InstigatedBy :type "Controller Object Reference") (DamageCauser :type "Actor Object Reference"))
  (`self.SpawnDamagePopup` Damage)
  (bind _output_get (set `self.CurrentHealth` (- (`self.CurrentHealth`) Damage)))
  (`self.OnHealthChanged` _output_get (`.CurrentAmount_20_1C1F45344E87F293D251F4BC53114A3C` (break `/Game/F_TowerAttributes` (`self.GetHealthAtrribute` (`self.Attributes`)))))
  (if (<= (`self.CurrentHealth`) 0.0)
    (`self.DestroyPlacedTile`)))

(event `/Game/I_Clickable.OnItemClicked`
  (bind _owning_tile (`self.Owning Tile`))
  (if (`KismetSystemLibrary.IsValid` _owning_tile)
    (`/Game/Hexagon/BP_BaseHexTile.OnTileClicked` _owning_tile)
    (bind _asbp_top_down_character (cast `/Game/TopDown/Blueprints/BP_TopDownCharacter` (`GameplayStatics.GetPlayerCharacter` 0)))
    (set `/Game/TopDown/Blueprints/BP_TopDownCharacter.SelectedTile` _owning_tile _asbp_top_down_character)
    (else
      (`KismetSystemLibrary.PrintString` "No owning tile set" true true (struct :`R` 1.0 :`G` 0.015484 :`A` 1.0)))))

(event `DestroyPlacedTile`
  (bind _owning_tile (`self.Owning Tile`))
  (set `/Game/Hexagon/BP_BaseHexTile.PlacedTile` null _owning_tile)
  (`/Game/Hexagon/BP_HexGrid.TowerEaten` (`/Game/Hexagon/BP_BaseHexTile.Grid Generator Ref` _owning_tile) self)
  (`self.OnTowerDeath`)
  (`self.K2_DestroyActor`))

(event `SpawnDamagePopup`
  (params (DamageToDisplay :type "Float (double-precision)"))
  (bind (_returnvalue_x _returnvalue_y _returnvalue_z) (`KismetMathLibrary.BreakVector` (`self.K2_GetActorLocation`)))
  (bind _returnvalue (`|SpawnActorFromClass` "/Game/UI/BP_HealthPopupNotify.BP_HealthPopupNotify_C" (`KismetMathLibrary.MakeTransform` (`KismetMathLibrary.MakeVector` _returnvalue_x _returnvalue_y (+ _returnvalue_z 450.0))) "Undefined" "MultiplyWithRoot" null null))
  (`/Game/UI/BP_HealthPopupNotify.Initialise` _returnvalue DamageToDisplay))

(event `RotateHealthWidget`
  (params (NewRotation :type "Rotator Structure"))
  (`SceneComponent.K2_SetWorldRotation` (`self.WidgetHealth`) (`KismetMathLibrary.MakeRotator` 0.0 0.0 (- NewRotation_Yaw 180.0)) false false))

(fn `GetHealthAtrribute`
  (params (Attributes :type "Array of /Game/F_TowerAttributes Structure"))
  (returns (HealthAttribute :type "/Game/F_TowerAttributes Structure"))
  (for _array_element Attributes
    (if (`|EnumEquality` (`.AttributeType_27_401693E34E656CC35BD962A172F4A6D6` (break `/Game/F_TowerAttributes` _array_element)) "NewEnumerator0")
      (return _array_element))))

(fn `OnTowerDeath`
  (`self.OnTowerDied`))

(fn `UpdateCurrentMultiplier`
  (params (`Increase?` :type Boolean) (Amount :type "Float (double-precision)"))
  (if `Increase?`
    (set `self.CurrentMultiplier` (+ (`self.CurrentMultiplier`) Amount))
    (else
      (set `self.CurrentMultiplier` (- (`self.CurrentMultiplier`) Amount)))))

(fn `UpgradeStat`
  (params (Index :type Integer))
  (bind _attributes (`self.Attributes`))
  (bind (_attributetype _upgradecost _currentamount _upgradelevel _upgradeamount _uiinformation) (break `/Game/F_TowerAttributes` (`|GetArrayItem` _attributes Index)))
  (`KismetArrayLibrary.Array_Set` _attributes Index (make `/Game/F_TowerAttributes` _attributetype (`KismetMathLibrary.Conv_IntToDouble` (`KismetMathLibrary.Round` (* _upgradecost 1.25))) (+ _currentamount _upgradeamount) (+ _upgradelevel 1) _upgradeamount _uiinformation))
  (`self.OnAttributesChanged`)
  (if (`|EnumEquality` _attributetype "NewEnumerator0")
    (bind _output_get (set `self.CurrentHealth` (+ (`self.CurrentHealth`) _upgradeamount)))
    (`self.OnHealthChanged` _output_get _currentamount)))

(fn `UserConstructionScript`)