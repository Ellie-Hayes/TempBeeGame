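; BP_Nectar is a nectar pickup in the Flower Fields tower area that bobs up and down until collected.
; Shortly after BeginPlay, a looping event alternates two timelines through a FlipFlop, lerping the actor up, then down, from its location at the start of each pass.
; A Collect event spawns a honey blast Niagara effect at the actor and destroys it a tick later.
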(event `self.ReceiveBeginPlay`
  (`KismetSystemLibrary.Delay` 0.5)
  (`self.Float Up and Down`))

(event `Float Up and Down`
  ;[1 1 1] Bounce up and Down
  (set `self.OriginalLocation` (`self.K2_GetActorLocation`))
  (`KismetSystemLibrary.DelayUntilNextTick`)
  (`/Engine/EditorBlueprintResources/StandardMacros.FlipFlop`
    (:`A`
      (bind (_direction _newtrack_0) (`Timeline|Timeline` :!via `PlayFromStart`)
        (:`Update`
          (`self.K2_SetActorLocation` (`KismetMathLibrary.VLerp` (`self.OriginalLocation`) (+ (`self.OriginalLocation`) (0.0 0.0 75.0)) _newtrack_0)))
        (:`Finished`
          (`self.Float Up and Down`))))
    (:`B`
      (bind (_direction_2 _newtrack_0_2) (`Timeline|Timeline_0` :!via `PlayFromStart`)
        (:`Update`
          (`self.K2_SetActorLocation` (`KismetMathLibrary.VLerp` (`self.OriginalLocation`) (+ (`self.OriginalLocation`) (0.0 0.0 -75.0)) _newtrack_0_2)))
        (:`Finished`
          (`self.Float Up and Down`))))))

(event `Collect`
  (`NiagaraFunctionLibrary.SpawnSystemAtLocation` "/Game/VFX/ActiveEffects/Systems/NS_HoneyBlast1.NS_HoneyBlast1" (`self.K2_GetActorLocation`))
  (`KismetSystemLibrary.DelayUntilNextTick`)
  (`self.K2_DestroyActor`))

(fn `UserConstructionScript`)