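; BP_BaseTower is a tower Blueprint that holds a multiplier value and provides a function to adjust it.
; UpdateTowerMultiplier adds Amount when Increase is true; otherwise it sets the multiplier to Amount minus the current value, not the reverse.
; The result is clamped to a minimum of one.
; The event graph and construction script add no behavior of their own.
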(fn `UpdateTowerMultiplier`
  (params (`Increase?` :type Boolean) (Amount :type "Float (double-precision)"))
  (if `Increase?`
    (set `self.CurrentMultiplier_0` (+ Amount (`self.CurrentMultiplier_0`)))
    (else
      (set `self.CurrentMultiplier_0` (- Amount (`self.CurrentMultiplier_0`)))))
  (if (<= (`self.CurrentMultiplier_0`) 1.0)
    (set `self.CurrentMultiplier_0` 1.0)))

(fn `UserConstructionScript`
  (`parent.UserConstructionScript`))