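; Royal Jelly Booster is a tower that boosts one linked tower.
; Selecting that tower raises its multiplier, resumes its healing timer and spawns a bee given the booster as home and the tower as target.
; Deselecting lowers the multiplier, pauses healing, clears the link and destroys the bee.
; An area boost for neighbouring placed tiles exists only as unconnected logic, leaving UpdateTowersBoosted empty.
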(event `self.Initialise`
  (params (OwningTile :type "/Game/Hexagon/BP_BaseHexTile Object Reference"))
  (bind _output_get (set `self.Owning Tile` OwningTile))
  (set `self.GridRef` (`/Game/Hexagon/BP_BaseHexTile.Grid Generator Ref` _output_get)))

(fn `TowerDeselected`
  (bind _asbp_base_placeable (cast `/Game/Towers/BP_BasePlaceable` (`self.LinkedTower`)))
  (`self.UpdateCurrentMultiplier` _asbp_base_placeable false (`self.BoostMultiplierAmount`))
  (set `self.ConnectedToTower` false)
  (set `self.LinkedTower` null)
  (`KismetSystemLibrary.K2_PauseTimerHandle` (`/Game/Towers/BP_BasePlaceable.Healing Timer` _asbp_base_placeable))
  (`self.K2_DestroyActor` (`self.Bee`)))

(fn `TowerSelected`
  (bind _linkedtower (`self.LinkedTower`))
  (bind _returnvalue (`self.GetTransform` self))
  (bind _asbp_base_placeable (cast `/Game/Towers/BP_BasePlaceable` _linkedtower))
  (`self.UpdateCurrentMultiplier` _asbp_base_placeable true (`self.BoostMultiplierAmount`))
  (set `self.ConnectedToTower` true)
  (`KismetSystemLibrary.K2_UnPauseTimerHandle` (`/Game/Towers/BP_BasePlaceable.Healing Timer` _asbp_base_placeable))
  (bind _returnvalue_2 (`|SpawnActorFromClass` "/Game/BP_Bee.BP_Bee_C" _returnvalue "Undefined" "MultiplyWithRoot" null null))
  (set `self.Bee` _returnvalue_2)
  (set `/Game/BP_Bee.Home Location` (.location _returnvalue) _returnvalue_2)
  (set `/Game/BP_Bee.Target Location` (`self.K2_GetActorLocation` _linkedtower) _returnvalue_2))

(fn `UpdateTowersBoosted`
  (params (PlacedTower :type "/Game/Towers/BP_BasePlaceable Object Reference")))

(fn `UserConstructionScript`
  (`parent.UserConstructionScript`))