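; Single-target turret tower that fires homing bullets at enemies while it is connected to a hive.
; PawnSensing, with its sight radius set in the construction script, detects pawns tagged Enemy and turns Cube1 toward them with pitch zeroed.
; Bullets spawn at the Arrow, with damage taken from an attribute scaled by CurrentMultiplier.
; A CanShoot flag and Delay gate the fire rate, with a non-default multiplier adjusting the cooldown.
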(event `self.ReceiveBeginPlay`)

(event `Update Stat`)

(event `self.PawnSensing.OnSeePawn`
  (params (Pawn :type "Pawn Object Reference"))
  (bind _currentmultiplier (`self.CurrentMultiplier`))
  (bind ((`AttributeType_27_401693E34E656CC35BD962A172F4A6D6` _attributetype) (`CurrentAmount_20_1C1F45344E87F293D251F4BC53114A3C` _currentamount)) (break `/Game/F_TowerAttributes` (`|GetArrayItem` (`self.Attributes`) 1)))
  (bind (_returnvalue_roll _returnvalue_pitch _returnvalue_yaw) (`KismetMathLibrary.BreakRotator` (`KismetMathLibrary.FindLookAtRotation` (`SceneComponent.K2_GetComponentLocation` (`self.Cube1`)) (`self.K2_GetActorLocation` Pawn))))
  (if (`self.ConnectedToHive`)
    (if (`self.ActorHasTag` Pawn "Enemy")
      (`SceneComponent.K2_SetWorldRotation` (`self.Cube1`) (`KismetMathLibrary.MakeRotator` _returnvalue_roll 0.0 _returnvalue_yaw) false false)
      (if (`self.CanShoot?`)
        (bind _returnvalue (`|SpawnActorFromClass` "/Game/TD_Prototipings/BP_Bullet.BP_Bullet_C" (`SceneComponent.K2_GetComponentToWorld` (`self.Arrow`)) "Undefined" "MultiplyWithRoot" null null))
        (set `ProjectileMovementComponent.HomingTargetComponent` (`Actor.RootComponent` Pawn) (`/Game/TD_Prototipings/BP_Bullet.ProjectileMovement` _returnvalue))
        (`/Game/TD_Prototipings/BP_Bullet.Initialise` _returnvalue (* (`self.CurrentMultiplier`) (`.CurrentAmount_20_1C1F45344E87F293D251F4BC53114A3C` (break `/Game/F_TowerAttributes` (`|GetArrayItem` (`self.Attributes`) 2)))) Pawn)
        (set `self.CanShoot?` false)
        (if (== _currentmultiplier 1.0)
          (`KismetSystemLibrary.Delay` _currentamount)
          (else
            (`KismetSystemLibrary.Delay` (* _currentamount (/ (- 100.0 (* _currentmultiplier (`self.Multiplier Effecting Number Mega Maths_44`))) 100.0)))))
        (set `self.CanShoot?` true)
        (`KismetSystemLibrary.PrintString` (`KismetStringLibrary.Conv_DoubleToString` _currentamount))))))

(fn `UpdateCurrentMultiplier`
  (params (`Increase?` :type Boolean) (Amount :type "Float (double-precision)"))
  (`parent.UpdateCurrentMultiplier` `Increase?` Amount))

(fn `UpdateTowerMultiplier`
  (params (`Increase?` :type Boolean) (Amount :type "Float (double-precision)"))
  (`parent.UpdateTowerMultiplier` `Increase?` Amount))

(fn `UserConstructionScript`
  (`parent.UserConstructionScript`)
  (set `PawnSensingComponent.SightRadius` (`self.Sight Radius`) (`self.PawnSensing`)))