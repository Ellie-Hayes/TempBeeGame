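; BP_Dog is a Hive tower pawn that shuttles between flower fields and its owner, though no nectar is actually transferred here.
; BeginPlay caches all BP_FlowerField actors once, then starts CollectNectar, which uses AIMoveTo to visit each in array order after a one-second delay.
; After the last field or a failed move, ReturnHome moves to the owner, then restarts collection whether that move succeeds or fails.
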(event `self.ReceiveBeginPlay`
  ;[1 1 1] Update All Actors Everytime A Flower Field is Placed
  (bind _outactors (`GameplayStatics.GetAllActorsOfClass` "/Game/Towers/FlowerFields/BP_FlowerField.BP_FlowerField_C"))
  (bind _output_get (set `self.FlowerField` _outactors))
  (set `self.Max Number Of Towers` (`KismetArrayLibrary.Array_Length` _output_get))
  (`KismetSystemLibrary.DelayUntilNextTick`)
  (`self.CollectNectar`))

(event `CollectNectar`
  (`KismetSystemLibrary.Delay` 1.0)
  (`|AIMoveTo` self (0.0 0.0 0.0) (`|GetArrayItem` (`self.FlowerField`) (`self.Integer`))
    (:`then`
      (`KismetSystemLibrary.PrintString` "Hello"))
    (:`OnSuccess`
      (bind _result (`/Engine/EditorBlueprintResources/StandardMacros.IncrementInt` (`self.Integer`))
        (:`  `
          (if (== _result (`self.Max Number Of Towers`))
            (set `self.Integer` 0)
            (`self.ReturnHome`)
            (else
              (`self.CollectNectar`))))))
    (:`OnFail`
      (`self.ReturnHome`))))

(event `ReturnHome`
  (`|AIMoveTo` self (0.0 0.0 0.0) (`self.GetOwner`)
    (:`OnSuccess`
      _)
    (:`OnFail`
      _))
  (`self.CollectNectar`))

(fn `UserConstructionScript`)