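; BP_Doggo is a hive-tower actor that patrols every BP_FlowerField in the level, resetting the nectar of each field it reaches.
; BeginPlay caches the fields and a currently unused resource generator reference, then unpauses one tick later.
; Tick moves it at constant speed in XY, facing the target field.
; Within range, it calls ResetNectar every tick while a one-second Delay runs, then advances the looping index.
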(event `self.ReceiveBeginPlay`
  (set `self.Paused` true)
  (bind _returnvalue (`GameplayStatics.GetActorOfClass` "/Game/Towers/BP_BaseResourceGenerator.BP_BaseResourceGenerator_C"))
  (set `self.BP_HiveRef` _returnvalue)
  (bind _outactors (`GameplayStatics.GetAllActorsOfClass` "/Game/Towers/FlowerFields/BP_FlowerField.BP_FlowerField_C"))
  (bind _output_get (set `self.FlowerFieldArray` _outactors))
  (set `self.MaxFlowerFieldInt` (`KismetArrayLibrary.Array_Length` _output_get))
  (`KismetSystemLibrary.DelayUntilNextTick`)
  (set `self.Paused` false))

(event `self.ReceiveTick`
  (params (DeltaSeconds :type "Float (single-precision)"))
  (bind (_returnvalue_x _returnvalue_y _returnvalue_z) (`KismetMathLibrary.BreakVector` (`self.K2_GetActorLocation`)))
  (bind (_returnvalue_x_2 _returnvalue_y_2 _returnvalue_z_2) (`KismetMathLibrary.BreakVector` (`self.K2_GetActorLocation`)))
  (bind (_returnvalue_x_3 _returnvalue_y_3) (`KismetMathLibrary.BreakVector` (`self.K2_GetActorLocation`)))
  (bind (_returnvalue_x_4 _returnvalue_y_4) (`KismetMathLibrary.BreakVector` (`self.K2_GetActorLocation` (`|GetArrayItem` (`self.FlowerFieldArray`) (`self.CurrentFlowerField`)))))
  (bind (_returnvalue_x_5 _returnvalue_y_5) (`KismetMathLibrary.BreakVector` (`self.K2_GetActorLocation` (`|GetArrayItem` (`self.FlowerFieldArray`) (`self.CurrentFlowerField`)))))
  (bind (_returnvalue_x_6 _returnvalue_y_6) (`KismetMathLibrary.BreakVector` (`self.K2_GetActorLocation` (`|GetArrayItem` (`self.FlowerFieldArray`) (`self.CurrentFlowerField`)))))
  ;[1 1 1] IsPaused?
  (if (not (`self.Paused`))
    (`self.K2_SetActorLocation` (`KismetMathLibrary.VInterpTo_Constant` (`KismetMathLibrary.MakeVector` _returnvalue_x_2 _returnvalue_y_2 _returnvalue_z_2) (`KismetMathLibrary.MakeVector` _returnvalue_x_5 _returnvalue_y_5 _returnvalue_z_2) DeltaSeconds (`self.Interp Speed`)) false true)
    (`self.K2_SetActorRotation` (`KismetMathLibrary.FindLookAtRotation` (`KismetMathLibrary.MakeVector` _returnvalue_x_3 _returnvalue_y_3) (`KismetMathLibrary.MakeVector` _returnvalue_x_6 _returnvalue_y_6)))
    (if (<= (`KismetMathLibrary.Vector_Distance` (`KismetMathLibrary.MakeVector` _returnvalue_x _returnvalue_y _returnvalue_z) (`KismetMathLibrary.MakeVector` _returnvalue_x_4 _returnvalue_y_4 _returnvalue_z)) 5.0)
      (`/Game/Towers/FlowerFields/BP_FlowerField.ResetNectar` (`|GetArrayItem` (`self.FlowerFieldArray`) (`self.CurrentFlowerField`)))
      (`KismetSystemLibrary.Delay` 1.0)
      (bind _result (`/Engine/EditorBlueprintResources/StandardMacros.IncrementInt` (`self.CurrentFlowerField`))
        (:`  `
          (if (>= _result (`self.MaxFlowerFieldInt`))
            (set `self.CurrentFlowerField` 0)))))))

(fn `UserConstructionScript`)