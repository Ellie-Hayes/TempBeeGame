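; BP_Dogg is a Hive tower pawn that uses AI movement to head for a flower field to collect nectar.
; On BeginPlay it caches all BP_FlowerField actors and their count, then calls CollectNectar once.
; CollectNectar moves toward the field at the current index and, on success, advances that index with wraparound.
; The graph neither repeats the move nor refreshes the field list afterward.
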(event `self.ReceiveBeginPlay`
  ;[1 1 1] Update All Actors Everytime A Flower Field is Placed
  (bind _outactors (`GameplayStatics.GetAllActorsOfClass` "/Game/Towers/FlowerField/BP_FlowerField.BP_FlowerField_C"))
  (bind _output_get (set `self.FlowerField` _outactors))
  (set `self.MaxNumberOfTowers` (`KismetArrayLibrary.Array_Length` _output_get))
  (`self.CollectNectar`))

(event `CollectNectar`
  (`|AIMoveTo` self (`self.K2_GetActorLocation`) (`|GetArrayItem` (`self.FlowerField`) (`self.Integer`))
    (:`OnSuccess`
      (bind _result (`/Engine/EditorBlueprintResources/StandardMacros.IncrementInt` (`self.Integer`))
        (:`  `
          (if (== _result (`self.MaxNumberOfTowers`))
            (set `self.Integer` 0)))))))

(fn `UserConstructionScript`)