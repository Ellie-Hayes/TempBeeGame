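; Actor component that shows a scaffolding preview when the cursor hovers over an empty hex tile.
; On BeginPlay it binds to its owner's cursor-over events.
; Hover spawns BP_Scaffolding at the tile's transform, only for an exact BP_BaseHexTile class with no valid PlacedTile, and cursor exit destroys it.
; Despite the component's name, no outline is drawn, and an older desaturated-material hover highlight remains as disconnected nodes.
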(event `self.ReceiveBeginPlay`
  (bind _returnvalue (`self.GetOwner`))
  (add `Actor.OnBeginCursorOver` _returnvalue (`|CreateDelegate` :!event `Cursor Over`))
  (add `Actor.OnEndCursorOver` _returnvalue (`|CreateDelegate` :!event `ResetMaterial`)))

(event `Cursor Over`
  (params (TouchedActor :type "Actor Object Reference"))
  (bind _asbp_base_hex_tile (cast `/Game/Hexagon/BP_BaseHexTile` TouchedActor))
  (if (and (not (`KismetSystemLibrary.IsValid` (`/Game/Hexagon/BP_BaseHexTile.PlacedTile` _asbp_base_hex_tile))) (== (`GameplayStatics.GetObjectClass` TouchedActor) "/Game/Hexagon/BP_BaseHexTile.BP_BaseHexTile_C") (not (== (`GameplayStatics.GetObjectClass` TouchedActor) "/Game/Towers/BP_BaseResourceGenerator.BP_BaseResourceGenerator_C")))
    (bind _returnvalue (`|SpawnActorFromClass` "/Game/Scaffolding/BP_Scaffolding.BP_Scaffolding_C" (`Actor.GetTransform` TouchedActor) "Undefined" "MultiplyWithRoot" null null))
    (set `self.NewVar` _returnvalue)))

(event `ResetMaterial`
  (params (TouchedActor :type "Actor Object Reference"))
  (bind _newvar (`self.NewVar`))
  (`/Engine/EditorBlueprintResources/StandardMacros.IsValid` _newvar
    (:`Is Valid`
      (`Actor.K2_DestroyActor` _newvar))))