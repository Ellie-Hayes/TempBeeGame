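; BP_Granade is a grenade actor that deals area damage on impact and leaves a honey splat effect.
; Its collision sphere ignores the owner while moving, and Initialise supplies the damage value.
; On Hit it spawns the Niagara splat, sphere-traces the damage radius for objects, applies flat damage per hit result, and destroys itself.
; A radial damage-with-falloff node remains unconnected.
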(event `self.ReceiveBeginPlay`
  (`PrimitiveComponent.IgnoreActorWhenMoving` (`self.Sphere1`) (`self.GetOwner`) true))

(event `Initialise`
  (params (Damage :type "Float (double-precision)"))
  (set `self.Damage` Damage))

(event `self.ReceiveHit`
  (params (MyComp :type "PrimitiveComponent Object Reference") (Other :type "Actor Object Reference") (OtherComp :type "PrimitiveComponent Object Reference") (bSelfMoved :type Boolean) (HitLocation :type "Vector Structure") (HitNormal :type "Vector Structure") (NormalImpulse :type "Vector Structure") (Hit :type "HitResult Structure (by ref)"))
  (`NiagaraFunctionLibrary.SpawnSystemAtLocation` "/Game/VFX/ActiveEffects/Systems/NS_HoneySplat.NS_HoneySplat" HitLocation)
  (bind _outhits (`KismetSystemLibrary.SphereTraceMultiForObjects` HitLocation HitLocation (`self.Damage Radius`) (`self.Object Types`)))
  (for _array_element _outhits
    (`GameplayStatics.ApplyDamage` (`.HitActor` (`GameplayStatics.BreakHitResult` _array_element)) (`self.Damage`))
    (`self.K2_DestroyActor` :!label _label))
  (goto _label))

(fn `UserConstructionScript`)