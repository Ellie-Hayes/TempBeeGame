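; BP_Pollen_Bomber is a mortar shooter that turns toward sensed pawns tagged "Enemy" and lobs BP_Granade projectiles at them.
; On sight it spawns a grenade at its Arrow, sets the launch velocity, then waits out a cooldown.
; MortarPrediction leads the target by velocity times distance over a fixed speed, then solves a custom-arc launch velocity.
; AddVectorRandomness only feeds a debug sphere, so the shot itself gets no scatter.
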(event `self.ReceiveBeginPlay`)

(event `self.PawnSensing.OnSeePawn`
  (params (Pawn :type "Pawn Object Reference"))
  (if (`self.ActorHasTag` Pawn "Enemy")
    (`self.K2_SetActorRotation` (`KismetMathLibrary.FindLookAtRotation` (`self.K2_GetActorLocation`) (`self.K2_GetActorLocation` Pawn)))
    (if (`self.CanShoot?`)
      (bind _velocity (`self.Mortar Prediction` Pawn))
      (set `self.Velocity` _velocity)
      (bind _returnvalue (`|SpawnActorFromClass` "/Game/TD_Prototipings/BP_Granade.BP_Granade_C" (`KismetMathLibrary.MakeTransform` (`SceneComponent.K2_GetComponentLocation` (`self.Arrow`))) "Undefined" "MultiplyWithRoot" null null))
      (`ProjectileMovementComponent.SetVelocityInLocalSpace` (`/Game/TD_Prototipings/BP_Granade.ProjectileMovement` _returnvalue) (`self.Velocity`))
      (set `self.CanShoot?` false)
      (`KismetSystemLibrary.Delay` (`self.Fire Cooldown`))
      (set `self.CanShoot?` true))))

(fn `Add Vector Randomness`
  (params (Vector :type "Vector Structure") (Randomness :type "Float (double-precision)") (`Use X` :type Boolean) (`Use Y` :type Boolean) (`Use Z` :type Boolean))
  (returns (`Randomness Return` :type "Vector Structure"))
  (bind _x (.x Vector))
  (bind _y (.y Vector))
  (bind _z (.z Vector))
  (bind _returnvalue (* Randomness -1.0))
  (return (`KismetMathLibrary.MakeVector` (`KismetMathLibrary.SelectFloat` (+ (`KismetMathLibrary.RandomFloatInRange` _returnvalue Randomness) _x) _x) (`KismetMathLibrary.SelectFloat` (+ (`KismetMathLibrary.RandomFloatInRange` _returnvalue Randomness) _y) _y) (`KismetMathLibrary.SelectFloat` (+ (`KismetMathLibrary.RandomFloatInRange` _returnvalue) _z) _z))))

(fn `Mortar Prediction`
  (params (`Target Actor` :type "Actor Object Reference"))
  (returns (Velocity :type "Vector Structure"))
  (locals (`Target Actor Velocity` :type "Vector Structure") (`Target Actor Location` :type "Vector Structure"))
  (bind _returnvalue (+ (`local.Target Actor Location`) (* (`local.Target Actor Velocity`) (/ (`KismetMathLibrary.Vector_Distance` (`local.Target Actor Location`) (`self.K2_GetActorLocation`)) 1200.0))))
  (set `local.Target Actor Velocity` (`self.GetVelocity` `Target Actor`))
  (set `local.Target Actor Location` (`self.K2_GetActorLocation` `Target Actor`))
  (`KismetSystemLibrary.DrawDebugSphere` _returnvalue 100.0 12 (struct :`R` 0.067444 :`G` 1.0 :`A` 1.0))
  (`KismetSystemLibrary.DrawDebugSphere` (`self.Add Vector Randomness` _returnvalue 0.0 true true true) 100.0 12 (struct :`R` 1.0 :`B` 0.087291 :`A` 1.0))
  (bind (_outlaunchvelocity _returnvalue_2) (`GameplayStatics.SuggestProjectileVelocity_CustomArc` (`SceneComponent.K2_GetComponentLocation` (`self.Arrow`)) _returnvalue))
  (if _returnvalue_2
    (return _outlaunchvelocity)))

(fn `UserConstructionScript`)