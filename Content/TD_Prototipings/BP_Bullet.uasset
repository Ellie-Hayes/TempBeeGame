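; BP_Bullet is a tower-defense prototype projectile that damages an enemy on contact with a honey-blast effect.
; Initialise stores damage and target.
; The first sphere overlap consumes a DoOnce, and only an Enemy-tagged actor triggers damage, Niagara blast and delayed destruction.
; A Timeline that would lerp the bullet toward its target and share that impact sequence is never triggered, so this graph does not move it.
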(event `Initialise`
  (params (NewDamage :type "Float (double-precision)") (NewTarget :type "Actor Object Reference"))
  (set `self.Damage` NewDamage)
  (set `self.Target` NewTarget))

(event `self.Sphere1.OnComponentBeginOverlap`
  (params (OverlappedComponent :type "PrimitiveComponent Object Reference") (OtherActor :type "Actor Object Reference") (OtherComp :type "PrimitiveComponent Object Reference") (OtherBodyIndex :type Integer) (bFromSweep :type Boolean) (SweepResult :type "HitResult Structure (by ref)"))
  (`/Engine/EditorBlueprintResources/StandardMacros.DoOnce` false
    (:`Completed`
      (if (`self.ActorHasTag` OtherActor "Enemy")
        (`GameplayStatics.ApplyDamage` OtherActor (`self.Damage`))
        (`ActorComponent.Deactivate` (`self.NS_HoneyBlast`))
        (`NiagaraFunctionLibrary.SpawnSystemAtLocation` "/Game/VFX/ActiveEffects/Systems/NS_HoneyBlast1.NS_HoneyBlast1" (`self.K2_GetActorLocation`))
        (`KismetSystemLibrary.Delay` 0.3)
        (`self.K2_DestroyActor`)))))

(fn `UserConstructionScript`)