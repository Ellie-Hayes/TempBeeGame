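; BP_Sticky_Honey is a prototype sticky honey zone that changes the movement speed of enemies inside its box.
; Box begin and end overlaps cast the other actor to BP_EnemyAIBase and apply a start or end speed value.
; It writes only MaxCustomMovementSpeed on CharacterMovement, which applies to custom movement mode, leaving MaxWalkSpeed untouched.
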(event `self.Box.OnComponentBeginOverlap`
  (params (OverlappedComponent :type "PrimitiveComponent Object Reference") (OtherActor :type "Actor Object Reference") (OtherComp :type "PrimitiveComponent Object Reference") (OtherBodyIndex :type Integer) (bFromSweep :type Boolean) (SweepResult :type "HitResult Structure (by ref)"))
  (bind _asbp_enemy_aibase (cast `/Game/EnemyAI/BP_EnemyAIBase` OtherActor))
  (bind _output_get (set `self.As BP Enemy AIBase` _asbp_enemy_aibase))
  (set `CharacterMovementComponent.MaxCustomMovementSpeed` (`self.Max Custom Movement SpeedStart`) (`Character.CharacterMovement` _output_get)))

(event `self.Box.OnComponentEndOverlap`
  (params (OverlappedComponent :type "PrimitiveComponent Object Reference") (OtherActor :type "Actor Object Reference") (OtherComp :type "PrimitiveComponent Object Reference") (OtherBodyIndex :type Integer))
  (bind _asbp_enemy_aibase (cast `/Game/EnemyAI/BP_EnemyAIBase` OtherActor))
  (bind _output_get (set `self.As BP Enemy AIBase` _asbp_enemy_aibase))
  (set `CharacterMovementComponent.MaxCustomMovementSpeed` (`self.Max Custom Movement SpeedEnd`) (`Character.CharacterMovement` _output_get)))

(fn `UserConstructionScript`)