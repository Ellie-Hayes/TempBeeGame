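; BP_BuffBullet is a tower defense prototype actor that buffs a turret overlapping its Box component.
; On begin overlap it casts to BP_Single_Turret, caches the reference, and writes its buff values to the turret's duration and bullet damage.
; End overlap writes the same values to the last cached turret without checking the leaving actor, so the buff is not reverted.
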(event `self.Box.OnComponentBeginOverlap`
  (params (OverlappedComponent :type "PrimitiveComponent Object Reference") (OtherActor :type "Actor Object Reference") (OtherComp :type "PrimitiveComponent Object Reference") (OtherBodyIndex :type Integer) (bFromSweep :type Boolean) (SweepResult :type "HitResult Structure (by ref)"))
  (bind _asbp_single_turret (cast `/Game/Towers/BP_Single_Turret` OtherActor))
  (bind _output_get (set `self.As BP Single Turret` _asbp_single_turret))
  (set `/Game/Towers/BP_Single_Turret.Duration_0` (`self.Duration Buff`) _output_get)
  (set `/Game/TD_Prototipings/BP_Bullet.Damege` (`self.Damege_Buff`) (`/Game/Towers/BP_Single_Turret.Bullet` _output_get)))

(event `self.Box.OnComponentEndOverlap`
  (params (OverlappedComponent :type "PrimitiveComponent Object Reference") (OtherActor :type "Actor Object Reference") (OtherComp :type "PrimitiveComponent Object Reference") (OtherBodyIndex :type Integer))
  (bind _as_bp_single_turret (`self.As BP Single Turret`))
  (set `/Game/Towers/BP_Single_Turret.Duration_0` (`self.Duration Buff`) _as_bp_single_turret)
  (set `/Game/TD_Prototipings/BP_Bullet.Damege` (`self.Damege_Buff`) (`/Game/Towers/BP_Single_Turret.Bullet` _as_bp_single_turret)))

(fn `UserConstructionScript`)