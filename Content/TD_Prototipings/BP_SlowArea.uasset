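; BP_SlowArea is a tower defense prototype area that slows enemies while they are inside its box.
; On box overlap, an actor tagged Enemy that casts to BP_BaseEnemy has its current max speed saved and its walk speed scaled by SlowAmountMultiplier.
; On exit, the walk speed is set back from OriginalSpeed, a single variable shared by all enemies and overwritten on each entry.
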(event `self.Box.OnComponentBeginOverlap`
  (params (OverlappedComponent :type "PrimitiveComponent Object Reference") (OtherActor :type "Actor Object Reference") (OtherComp :type "PrimitiveComponent Object Reference") (OtherBodyIndex :type Integer) (bFromSweep :type Boolean) (SweepResult :type "HitResult Structure (by ref)"))
  (if (`self.ActorHasTag` OtherActor "Enemy")
    (bind _asbp_base_enemy (cast `/Game/EnemyAI/BP_BaseEnemy` OtherActor))
    (bind _output_get (set `self.As BP Enemy AITest` _asbp_base_enemy))
    (set `self.Original Speed` (`MovementComponent.GetMaxSpeed` (`Character.CharacterMovement` _output_get)))
    (set `CharacterMovementComponent.MaxWalkSpeed` (* (`self.Original Speed`) (`self.Slow Amount Multiplier`)) (`Character.CharacterMovement` _output_get))))

(event `self.Box.OnComponentEndOverlap`
  (params (OverlappedComponent :type "PrimitiveComponent Object Reference") (OtherActor :type "Actor Object Reference") (OtherComp :type "PrimitiveComponent Object Reference") (OtherBodyIndex :type Integer))
  (if (`self.ActorHasTag` OtherActor "Enemy")
    (bind _asbp_base_enemy (cast `/Game/EnemyAI/BP_BaseEnemy` OtherActor))
    (set `CharacterMovementComponent.MaxWalkSpeed` (`self.Original Speed`) (`Character.CharacterMovement` _asbp_base_enemy))))

(fn `UserConstructionScript`)