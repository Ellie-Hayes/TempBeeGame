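; Turret actor for a tower-defense prototype that faces and fires at pawns it detects.
; PawnSensing's OnSeePawn snaps the whole actor's rotation toward the seen pawn.
; If CanShoot is set, it spawns a BP_Bullet at the Arrow component's transform, then uses the flag and a Delay as a fire-rate cooldown.
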(event `self.PawnSensing.OnSeePawn`
  (params (Pawn :type "Pawn Object Reference"))
  (`self.K2_SetActorRotation` (`KismetMathLibrary.FindLookAtRotation` (`self.K2_GetActorLocation`) (`self.K2_GetActorLocation` Pawn)))
  (if (`self.CanShoot?`)
    (`|SpawnActorFromClass` "/Game/TD_Prototipings/BP_Bullet.BP_Bullet_C" (`SceneComponent.K2_GetComponentToWorld` (`self.Arrow`)) "Undefined" "MultiplyWithRoot" null null)
    (set `self.CanShoot?` false)
    (`KismetSystemLibrary.Delay` (`self.Duration`))
    (set `self.CanShoot?` true)))

(fn `UserConstructionScript`)