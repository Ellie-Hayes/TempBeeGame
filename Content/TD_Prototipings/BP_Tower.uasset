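; BP_Tower is a prototype turret actor that automatically fires BP_Granade projectiles at pawns it detects.
; When PawnSensing sees a pawn and CanShoot is true, the tower snaps to face it, briefly waits, then spawns a grenade at its Arrow's transform.
; The CanShoot flag then blocks turning and firing until a cooldown set by Duration ends.
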(event `self.PawnSensing.OnSeePawn`
  (params (Pawn :type "Pawn Object Reference"))
  (if (`self.CanShoot?`)
    (`self.K2_SetActorRotation` (`KismetMathLibrary.FindLookAtRotation` (`self.K2_GetActorLocation`) (`self.K2_GetActorLocation` Pawn)))
    (`KismetSystemLibrary.Delay` 0.2)
    (`|SpawnActorFromClass` "/Game/TD_Prototipings/BP_Granade.BP_Granade_C" (`SceneComponent.K2_GetComponentToWorld` (`self.Arrow`)) "Undefined" "MultiplyWithRoot" null null)
    (set `self.CanShoot?` false)
    (`KismetSystemLibrary.Delay` (`self.Duration`))
    (set `self.CanShoot?` true)))

(fn `UserConstructionScript`)